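; BP_Unit is a networked character for turn-based combat, with team-colored text, highlighting and a cursor-facing ability range decal.
; Move commands use AIMoveTo, while a Tick gate totals distance walked and stops movement beyond the first ability's range.
; Damage passes through BPI_DamageTypes into attribute health, triggering multicast hit or knockdown montages, with OnRep damage numbers.
; GameState phase changes resolve knockdown and death on authority; destruction notifies the GameMode.
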(event `self.ReceiveTick`
  (params (DeltaSeconds :type "Float (single-precision)"))
  (`self.RotateDecal`)
  (`self.SetUnitFrame`)
  (`PrimitiveComponent.SetReceivesDecals` (`self.Mesh`) false)
  (`/Engine/EditorBlueprintResources/StandardMacros.Gate` true :!label _label
    (:`Exit`
      (`self.CalculateSteps`))))

(event `StartCountingSteps`
  (set `self.PreviousLocation` (`self.K2_GetActorLocation`))
  (set `self.CurrentWalkDistance` 0.0)
  (goto _label :!via `Open`))

(event `StopCountingSteps`
  (goto _label :!via `Close`))

(event `self.ReceiveBeginPlay`
  ;[1 1 1] Allow time to replicate
  (`KismetSystemLibrary.Delay` 0.2)
  (`self.InitUI`)
  ;[1 0 0] Check target function is empty should unit name be set here or on player controller if coming from a player state?
  (bind _asgs_turn_based (cast `/Game/Game/System/Gameplay/GS_TurnBased` (`GameplayStatics.GetGameState`)))
  (add `/Game/Game/System/Gameplay/GS_TurnBased.OnPhaseChanged` _asgs_turn_based (`|CreateDelegate` :!event `OnPhaseChanged`)))

(event `Command_Move`
  (params (DesiredLocation :type "Vector Structure"))
  (`self.SetMovementSpeed` DesiredLocation)
  (`|AIMoveTo` self DesiredLocation null
    (:`then`
      (bind _returnvalue (`/Game/Game/Blueprints/Abilities/Data/PDA_Action.GetUnitModifiedRange` (`|GetArrayItem` (`self.Abilities`)) self))
      (set `self.MaxMoveRange` _returnvalue)
      (`self.StartCountingSteps`))
    (:`OnSuccess`
      ;[1 0 0] Should this be generic (OnActionEnded?)
      (`self.OnMoveEnded` true)
      (`self.StopCountingSteps`))
    (:`OnFail`
      (`self.OnMoveEnded` false)
      (`self.StopCountingSteps`))))

(event `InitUI`
  (`|ExecutionSequence`
    (:`then_0`
      ;[1 0 0] Maybe move onto Attributes component!? update WB_AttributeBar to use Owning pawn
      (bind _aswb_unit_hudframe (cast `/Game/Game/UI/Gameplay/Unit/WB_UnitHUDFrame` (`WidgetComponent.GetWidget` (`self.Widget_UnitHUD`))))
      (`/Game/Game/UI/Gameplay/Unit/WB_UnitHUDFrame.SetUnit` _aswb_unit_hudframe self))))

(event `MULTII_Idle`
  ;[1 0 0] Comment
  (`GameplayStatics.SpawnSoundAttached` null (`self.Mesh`) "None" (0.0 0.0 0.0) (struct) "KeepRelativeOffset" false 1.0 1.0 0.0 null null)
  (`|PlayMontage` (`self.Mesh`)))

(event `MULTI_OnHit`
  ;[1 0 0] Comment
  (`GameplayStatics.SpawnSoundAttached` null (`self.Mesh`) "None" (0.0 0.0 0.0) (struct) "KeepRelativeOffset" false 1.0 1.0 0.0 null null)
  (`|PlayMontage` (`self.Mesh`)))

(event `MULTI_Death`
  ;[1 0 0] Comment
  (`GameplayStatics.SpawnSoundAttached` null (`self.Mesh`) "None" (0.0 0.0 0.0) (struct) "KeepRelativeOffset" false 1.0 1.0 0.0 null null)
  (`|PlayMontage` (`self.Mesh`) "/Game/Characters/Mannequins/Animations/Manny/Deaths_Gut_Shot_Montage.Deaths_Gut_Shot_Montage"))

(event `MULTI_Taunt`
  ;[1 0 0] Comment
  (`GameplayStatics.SpawnSoundAttached` null (`self.Mesh`) "None" (0.0 0.0 0.0) (struct) "KeepRelativeOffset" false 1.0 1.0 0.0 null null)
  (`|PlayMontage` (`self.Mesh`)))

(event `MULTI_KnockDown`
  ;[1 0 0] Comment
  (`GameplayStatics.SpawnSoundAttached` null (`self.Mesh`) "None" (0.0 0.0 0.0) (struct) "KeepRelativeOffset" false 1.0 1.0 0.0 null null)
  (`|PlayMontage` (`self.Mesh`)))

(event `self.ReceiveAnyDamage`
  (params (Damage :type "Float (single-precision)") (DamageType :type "DamageType Object Reference") (InstigatedBy :type "Controller Object Reference") (DamageCauser :type "Actor Object Reference"))
  (bind _ac_attributes (`self.AC_Attributes`))
  ;[1 0 0] Ive added damage event to use tags but this is before deciding on moving to a component
  (`/Engine/EditorBlueprintResources/StandardMacros.DoOnce` false :!label _label_2
    (:`Completed`
      (set `self.Damage Causer` DamageCauser)
      (if (`KismetSystemLibrary.DoesImplementInterface` DamageType "/Game/Game/Blueprints/DamageTypes/Interface/BPI_DamageTypes.BPI_DamageTypes_C")
        (bind (_calculateddamage _damagetype) (message `/Game/Game/Blueprints/DamageTypes/Interface/BPI_DamageTypes.UpdateDamage` DamageType Damage DamageCauser self))
        (set `self.LastDamageReceived` _calculateddamage)
        (else
          (set `self.LastDamageReceived` Damage)))
      (set `/Game/Game/System/Components/AC_Attributes.Health` (`KismetMathLibrary.FClamp` (- (`/Game/Game/System/Components/AC_Attributes.Health` _ac_attributes) (`self.LastDamageReceived`)) 0.0 (`/Game/Game/System/Components/AC_Attributes.MaxHealth` _ac_attributes)) _ac_attributes)
      (if (<= (`/Game/Game/System/Components/AC_Attributes.Health` (`self.AC_Attributes`)) 0.0)
        (`self.MULTI_KnockDown`)
        (else
          (`self.MULTI_OnHit`)
          (`KismetSystemLibrary.Delay` 0.2)
          (`self.DamageCooldown`))))))

(event `DamageCooldown`
  ;[1 0 0] Ive added damage event to use tags but this is before deciding on moving to a component
  (goto _label_2 :!via `Reset`))

(event `OnPhaseChanged`
  (params (Phase :type "/Game/Game/System/Enums/EPhase Enum" :default "NewEnumerator5"))
  (`/Engine/EditorBlueprintResources/ActorMacros.Switch Has Authority`
    (:`Authority`
      (switch `/Game/Game/System/Enums/EPhase` Phase
        (:`NewEnumerator2`
          ;[1 0 0] Set knockdown state maybe play animation? Maybe be a status effect on unit?
          (if (<= (`/Game/Game/System/Components/AC_Attributes.Health` (`self.AC_Attributes`)) 0.0)
            (`/Game/Game/System/Components/AC_GameplayTags.RemoveGameplayTag` :`self` (`self.AC_GameplayTags`) :`TagToRemove` (struct :`TagName` "State.Knockdown"))
            (`self.MULTI_KnockDown`)))
        (:`NewEnumerator3`
          (bind _attributefound (`/Game/Game/System/Components/AC_Attributes.GetAttributeFromTag` (`self.AC_Attributes`) (struct :`TagName` "Attribute.Health")))
          (if (<= (`.Curent_17_4F1F242B4B6319F1A1C212A3DDC2FAD3` (break `/Game/Game/System/Structs/FAttributeData` _attributefound)) 0.0)
            (`/Engine/EditorBlueprintResources/StandardMacros.DoOnce` false
              (:`Completed`
                (`self.MULTI_Death`)
                (set `/Game/Game/System/Gameplay/PC_TurnBased.IsUnitDead` true (`self.CommandController`))))))))))

(event `self.ReceiveDestroyed`
  (bind _asgm_turn_based (cast `/Game/Game/System/Gameplay/GM_TurnBased` (`GameplayStatics.GetGameMode`)))
  (`/Game/Game/System/Gameplay/GM_TurnBased.OnUnitDied` _asgm_turn_based self (`self.Damage Causer`)))

(event `/Game/Game/System/Interfaces/BPI_Animation.AnimateUnit`
  (params (Animation :type "GameplayTag Structure"))
  ;[1 0 0] Send Message for AnimateUnit
)

(event `/Game/Game/System/Interfaces/BPI_Animation.SignalAnimationEvent`
  (params (Animation :type "GameplayTag Structure") (Notify :type Name))
  ;[1 0 0] CallOnAnimationEvent add animation component and call to event dispatcher
)

(event `/Game/Game/System/Interfaces/BPI_Animation.SignalAnimationEnd`
  (params (Animation :type "GameplayTag Structure"))
  ;[1 0 0] Call OnAnimationEnd
)

(fn `CalculateSteps`
  (bind _output_get (set `self.CurrentWalkDistance` (+ (`self.CurrentWalkDistance`) (`KismetMathLibrary.Vector_Distance` (`self.K2_GetActorLocation`) (`self.PreviousLocation`)))))
  (set `self.PreviousLocation` (`self.K2_GetActorLocation`))
  (if (> _output_get (`self.MaxMoveRange`))
    (`Controller.StopMovement` (`AIBlueprintHelperLibrary.GetAIController` self))))

(fn `CheckTargets`)

(fn `GetLoadoutSelection`
  (returns (`Loadout Save` :type "/Game/Game/System/Save/SaveData_PlayerSettings Object Reference"))
  (`self.CommandController`
    (:`then`
      (return null))
    (:`else`)))

(fn `GetMesh`
  (returns (SkeletalMesh :type "SkeletalMeshComponent Object Reference"))
  (return (`self.Mesh`)))

(fn `HighlightUnit`
  (params (IsHighlighted :type Boolean))
  (`MeshComponent.SetOverlayMaterial` (`self.Mesh`) (select `bool` IsHighlighted :`true` "/Game/Game/Materials/M_SelectionOverlay.M_SelectionOverlay" :!type "MaterialInterface Object Reference")))

(fn `OnRep_LastDamageReceived`
  (bind _returnvalue (`|CreateWidget` "/Game/Game/UI/Gameplay/WB_DamageNumbers.WB_DamageNumbers_C" null self (`self.LastDamageReceived`) null))
  (`UserWidget.AddToViewport` _returnvalue 0))

(fn `RotateDecal`
  (bind (_returnvalue_roll _returnvalue_pitch _returnvalue_yaw) (`KismetMathLibrary.BreakRotator` (`KismetMathLibrary.FindLookAtRotation` (`self.K2_GetActorLocation`) (`.Location` (`GameplayStatics.BreakHitResult` (`PlayerController.GetHitResultUnderCursorByChannel` (`GameplayStatics.GetPlayerController` 0) "TraceTypeQuery1" true))))))
  (`SceneComponent.K2_SetWorldRotation` (`self.Decal_RangeIndicator`) (`KismetMathLibrary.MakeRotator` 0.0 -90.0 _returnvalue_yaw) false false))

(fn `SetMovementSpeed`
  (params (Destination :type "Vector Structure") (SprintRange :type "Float (double-precision)" :default 300.0))
  (set `CharacterMovementComponent.MaxWalkSpeed` (`KismetMathLibrary.SelectFloat` 600.0 300.0 (> (`KismetMathLibrary.Vector_Distance` Destination (`self.K2_GetActorLocation`)) SprintRange)) (`self.CharacterMovement`)))

(fn `SetRangeIndicator`
  (params (Range :type "Float (double-precision)") (Ability :type "/Game/Game/Blueprints/Abilities/Data/PDA_Action Object Reference"))
  (bind _decal_rangeindicator (`self.Decal_RangeIndicator`))
  (set `self.CurrentAbilityPreview` Ability)
  (if (> Range 0.0)
    (`SceneComponent.SetWorldScale3D` _decal_rangeindicator (`KismetMathLibrary.Conv_DoubleToVector` (/ Range 100.0)))
    (`SceneComponent.SetHiddenInGame` _decal_rangeindicator false false)
    (bind _currentabilitypreview (`self.CurrentAbilityPreview`)
      (:`then`
        (bind _returnvalue (`KismetMaterialLibrary.CreateDynamicMaterialInstance` (`DecalComponent.GetDecalMaterial` (`self.Decal_RangeIndicator`))))
        (`MaterialInstanceDynamic.SetScalarParameterValue` _returnvalue "Angle" (`/Game/Game/Blueprints/Abilities/Data/PDA_Action.Angle` _currentabilitypreview))
        (`DecalComponent.SetDecalMaterial` (`self.Decal_RangeIndicator`) _returnvalue))
      (:`else`))
    (else
      (`SceneComponent.SetHiddenInGame` _decal_rangeindicator true false))))

(fn `SetUnitFrame`
  (bind _textrender (`self.TextRender`))
  (bind _ac_attributes (`self.AC_Attributes`))
  (`TextRenderComponent.K2_SetText` _textrender (`KismetTextLibrary.Conv_DoubleToText` (`/Game/Game/System/Components/AC_Attributes.Haste` _ac_attributes) "HalfToEven"))
  (`TextRenderComponent.SetTextRenderColor` _textrender (`KismetMathLibrary.Conv_LinearColorToColor` (select `/Game/Game/System/Enums/ETeam` (`/Game/Game/System/Components/AC_Attributes.Team` _ac_attributes) :`NewEnumerator0` (struct :`R` 1.0 :`G` 1.0 :`B` 1.0 :`A` 1.0) :`NewEnumerator1` (struct :`R` 1.0 :`A` 1.0) :`NewEnumerator2` (struct :`B` 1.0 :`A` 1.0) :!type "LinearColor Structure"))))

(fn `UserConstructionScript`)