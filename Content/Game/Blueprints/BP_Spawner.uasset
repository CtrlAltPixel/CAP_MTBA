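; BP_Spawner is a turn-based game spawner that a player claims or releases by interacting with it.
; Interaction links spawner and PlayerController both ways; a player already holding one only releases it when interacting with an unclaimed spawner.
; A RepNotify on HasBeenAssigned recolors the cube to show claim state.
; It listens to GS_TurnBased phase changes and hides itself outside one specific phase, with no logic to unhide.
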(event `self.ReceiveBeginPlay`
  (bind _asgs_turn_based (cast `/Game/Game/System/GS_TurnBased` (`GameplayStatics.GetGameState`)))
  (add `/Game/Game/System/GS_TurnBased.OnPhaseChanged` _asgs_turn_based (delegate `OnPhaseChange`)))

(event `OnPhaseChange`
  (params (Phase :type "/Game/Game/System/Enums/EPhase Enum" :default "NewEnumerator5"))
  (if (`|EnumInequality` Phase "NewEnumerator5")
    (`self.SetActorHiddenInGame` true)))

(event `/Game/Game/System/BPI_Interaction.InteractWith`
  (params (PlayerController :type "/Game/Game/System/PC_TurnBased Object Reference"))
  (bind _currentlyinteractingplayer (`self.CurrentlyInteractingPlayer`))
  (set `self.CurrentlyInteractingPlayer` PlayerController)
  (if (`self.HasBeenAssigned`)
    (if (== (`self.CurrentlyInteractingPlayer`) (`self.AssignedPlayerController`))
      (set `self.HasBeenAssigned` false)
      (set `self.AssignedPlayerController` null)
      (set `/Game/Game/System/PC_TurnBased.Spawner` null (`self.CurrentlyInteractingPlayer`)))
    (else
      (bind _spawner (`/Game/Game/System/PC_TurnBased.Spawner` _currentlyinteractingplayer)
        (:`then`
          (set `/Game/Game/Blueprints/BP_Spawner.HasBeenAssigned` false _spawner)
          (set `/Game/Game/Blueprints/BP_Spawner.AssignedPlayerController` null _spawner)
          (set `/Game/Game/System/PC_TurnBased.Spawner` null (`self.CurrentlyInteractingPlayer`)))
        (:`else`
          (set `self.AssignedPlayerController` _currentlyinteractingplayer)
          (set `self.HasBeenAssigned` true)
          (set `/Game/Game/System/PC_TurnBased.Spawner` self (`self.CurrentlyInteractingPlayer`)))))))

(fn `OnRep_HasBeenAssigned`
  (if (`self.HasBeenAssigned`)
    (`MeshComponent.SetVectorParameterValueOnMaterials` (`self.Cube`) "Color" (`KismetMathLibrary.Conv_LinearColorToVector` (struct :`G` 0.5 :`B` 1.0 :`A` 1.0)))
    (else
      (`MeshComponent.SetVectorParameterValueOnMaterials` (`self.Cube`) "Color" (`KismetMathLibrary.Conv_LinearColorToVector` (struct :`R` 1.0 :`G` 0.5 :`A` 1.0))))))

(fn `UserConstructionScript`)