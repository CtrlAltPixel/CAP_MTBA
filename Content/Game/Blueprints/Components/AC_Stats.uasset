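; AC_Stats is a component holding an actor's combat and scoreboard stats.
; RepNotify functions fire three event dispatchers: health and resistances trigger OnUpdateHealth, resource triggers OnUpdateResource, and kills, deaths, assists, score and damage dealt trigger OnUpdateScore.
; On BeginPlay, the authority adds a random bonus to Haste.
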(event `self.ReceiveBeginPlay`
  (`/Engine/EditorBlueprintResources/ActorComponentMacros.Switch Has Authority`
    (:`Authority`
      (set `self.Haste` (+ (`self.Haste`) (`KismetMathLibrary.RandomFloatInRange` 0.0 60.0))))))

(fn `OnRep_Assists`
  (`self.OnUpdateScore`))

(fn `OnRep_DamageDealt`
  (`self.OnUpdateScore`))

(fn `OnRep_Deaths`
  (`self.OnUpdateScore`))

(fn `OnRep_Health`
  (`self.OnUpdateHealth`))

(fn `OnRep_Kills`
  (`self.OnUpdateScore`))

(fn `OnRep_MagicResist`
  (`self.OnUpdateHealth`))

(fn `OnRep_PhysicalResist`
  (`self.OnUpdateHealth`))

(fn `OnRep_Resource`
  (`self.OnUpdateResource`))

(fn `OnRep_Score`
  (`self.OnUpdateScore`))