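; Base weapon Blueprint driven by a WeaponData asset, which supplies its skeletal mesh and granted actions.
; BeginPlay applies the mesh when the data is valid.
; AddAction and RemoveAction register or unregister each of the data's actions with the owner's AC_Abilities component, and GetWeaponActions exposes that list.
; GetWeaponDamage is a stub returning zero, and the weapon XP component hook is an empty placeholder.
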(event `self.ReceiveBeginPlay`
  (bind _weapondata (`self.WeaponData`)
    (:`then`
      (`SkeletalMeshComponent.SetSkeletalMeshAsset` (`self.SkeletalMesh_Weapon`) (`/Game/Game/Blueprints/Equipment/Weapons/Data/PDA_Weapon.Mesh` _weapondata))
      ;[1 0 0] Playing with idea of a future XP Component (Not Created) for weapon types
      (`/Engine/EditorBlueprintResources/StandardMacros.IsValid` (`self.GetComponentByClass` (`self.GetOwner`) "/Script/Engine.ActorComponent")))
    (:`else`)))

(event `AddAction`
  (bind _returnvalue (`self.GetComponentByClass` (`self.GetOwner`) "/Game/Game/System/Components/AC_Abilities.AC_Abilities_C"))
  (`/Engine/EditorBlueprintResources/StandardMacros.IsValid` _returnvalue
    (:`Is Valid`
      (bind _weapondata (`self.WeaponData`)
        (:`then`
          (for _array_element (`/Game/Game/Blueprints/Equipment/Weapons/Data/PDA_Weapon.Actions` _weapondata)
            (`/Game/Game/System/Components/AC_Abilities.Add Action` _returnvalue _array_element)))
        (:`else`)))))

(event `RemoveAction`
  (bind _returnvalue (`self.GetComponentByClass` (`self.GetOwner`) "/Game/Game/System/Components/AC_Abilities.AC_Abilities_C"))
  (`/Engine/EditorBlueprintResources/StandardMacros.IsValid` _returnvalue
    (:`Is Valid`
      (bind _weapondata (`self.WeaponData`)
        (:`then`
          (for _array_element (`/Game/Game/Blueprints/Equipment/Weapons/Data/PDA_Weapon.Actions` _weapondata)
            (`/Game/Game/System/Components/AC_Abilities.Remove Action` _returnvalue _array_element)))
        (:`else`)))))

(fn `GetWeaponActions`
  (returns (NewParam :type "Array of /Game/Game/Blueprints/Abilities/Data/PDA_Action Object Reference"))
  (return (`/Game/Game/Blueprints/Equipment/Weapons/Data/PDA_Weapon.Actions` (`self.WeaponData`))))

(fn `GetWeaponDamage`
  (returns (WeaponDamage :type "Float (double-precision)"))
  (return 0.0))

(fn `NewFunction`)

(fn `UserConstructionScript`)