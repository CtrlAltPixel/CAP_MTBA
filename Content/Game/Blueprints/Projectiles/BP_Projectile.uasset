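; Projectile actor that flies straight along its forward vector and destroys itself on a qualifying overlap.
; BeginPlay sets the ProjectileMovement velocity from the forward vector scaled by ProjectileSpeed.
; When an overlapping actor passes an equality check, it spawns an emitter and plays a sound at its location, then destroys itself.
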(event `self.ReceiveBeginPlay`
  (set `MovementComponent.Velocity` (* (`self.GetActorForwardVector`) (`self.ProjectileSpeed`)) (`self.ProjectileMovement`)))

(event `self.ReceiveActorBeginOverlap`
  (params (OtherActor :type "Actor Object Reference"))
  (bind _returnvalue (`self.K2_GetActorLocation`))
  (if (== OtherActor null)
    (`GameplayStatics.SpawnEmitterAtLocation` null _returnvalue)
    (`GameplayStatics.PlaySoundAtLocation` null _returnvalue (struct) 1.0 1.0 0.0 null null null null)
    (`self.K2_DestroyActor`)))

(fn `UserConstructionScript`)