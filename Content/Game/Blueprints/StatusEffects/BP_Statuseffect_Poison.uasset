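; Poison status effect that damages the unit owning it each time its interval event fires.
; IntervalEffect casts the owner to BP_Unit, reaches PS_TurnBased through its instigator controller, and applies a fixed Health reduction via that player state's attributes component.
; The damage origin is the afflicted unit and its controller.
; Damage is a placeholder pending weapon and attribute calculation, and AI support remains an open question.
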(event `self.IntervalEffect`
  (bind _returnvalue (`self.GetOwner`))
  (bind _asbp_unit (cast `/Game/Game/Blueprints/Units/BP_Unit` _returnvalue))
  (bind _returnvalue_2 (`self.GetInstigatorController` _asbp_unit))
  ;[1 0 0] should attributes be player state or unit?
  (bind _asps_turn_based (cast `/Game/Game/System/Gameplay/PS_TurnBased` (`Controller.PlayerState` _returnvalue_2)))
  ;[1 0 0] Damage values will be calc from weapon and attriobutes
  (`/Game/Game/System/Components/AC_Attributes.ChangeAttribute` (`/Game/Game/System/Gameplay/PS_TurnBased.AC_Attributes` _asps_turn_based) (struct :`TagName` "Attribute.Health") -10.0 "NewEnumerator6" (make `/Game/Game/System/Structs/FOrigin` _returnvalue _returnvalue_2)))

(fn `UserConstructionScript`
  (`parent.UserConstructionScript`))