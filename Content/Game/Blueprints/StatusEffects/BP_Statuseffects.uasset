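; Base actor for turn-based status effects on a target unit; children supply the effect through ApplyStatusEffect.
; AttemptApplication checks the unit's required and preventing gameplay tags before applying.
; Game state phase changes reapply it without that check, on the data asset's phase and periodically during Planning.
; Each Respawn phase decrements the lifetime; at zero it removes itself from the unit's AC_StatusEffects component and destroys itself.
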(event `self.ReceiveBeginPlay`
  (bind _statuseffectdata (`self.StatusEffectData`)
    (:`then`
      (set `self.TurnCount` (`/Game/Game/Blueprints/StatusEffects/Data/PDA_StatusEffects.Lifetime` _statuseffectdata))
      (bind _asgs_turn_based (cast `/Game/Game/System/Gameplay/GS_TurnBased` (`GameplayStatics.GetGameState`)))
      (bind _output_get (set `self.As GS Turn Based` _asgs_turn_based))
      (add `/Game/Game/System/Gameplay/GS_TurnBased.OnPhaseChanged` _output_get (`|CreateDelegate` :!event `OnPhaseChange`)))
    (:`else`
      (`self.K2_DestroyActor`))))

(event `AttemptApplication`
  (bind _bsuccess_ (`self.CheckTagCondition`))
  (if _bsuccess_
    (`self.ApplyStatusEffect`)))

(event `ApplyStatusEffect`
  ;[1 1 1] Call from Children to apply tag per turn
)

(event `OnPhaseChange`
  (params (Phase :type "/Game/Game/System/Enums/EPhase Enum" :default "NewEnumerator5"))
  (`|ExecutionSequence`
    (:`then_0`
      (bind _statuseffectdata (`self.StatusEffectData`)
        (:`then`
          (if (`|EnumEquality` (`/Game/Game/Blueprints/StatusEffects/Data/PDA_StatusEffects.Phase` _statuseffectdata) Phase)
            (`self.ApplyStatusEffect`)))
        (:`else`)))
    (:`then_1`
      (switch `/Game/Game/System/Enums/EPhase` Phase
        (:`NewEnumerator1`
          (bind _statuseffectdata_2 (`self.StatusEffectData`)
            (:`then`
              (if (>= (`self.TickTime`) (`/Game/Game/Blueprints/StatusEffects/Data/PDA_StatusEffects.TickTime` _statuseffectdata_2))
                (set `self.TickTime` 0.0)
                (`self.ApplyStatusEffect`)
                (else
                  (`/Engine/EditorBlueprintResources/StandardMacros.IncrementFloat` (`self.TickTime`)))))
            (:`else`)))
        (:`NewEnumerator8`
          (bind _result (`/Engine/EditorBlueprintResources/StandardMacros.DecrementFloat` (`self.TurnCount`))
            (:`  `
              (if (<= _result 0.0)
                (`self.EndStatusEffect`)))))))))

(event `EndStatusEffect`
  (bind _returnvalue (`self.GetComponentByClass` (`self.TargetUnit`) "/Game/Game/System/Components/AC_StatusEffects.AC_StatusEffects_C"))
  (`/Engine/EditorBlueprintResources/StandardMacros.IsValid` _returnvalue
    (:`Is Valid`
      (`/Game/Game/System/Components/AC_StatusEffects.RemoveStatusEffect` _returnvalue self)
      (`self.K2_DestroyActor`))))

(fn `CheckTagCondition`
  (returns (`bSuccess?` :type Boolean))
  (bind _tagcontainer (`/Game/Game/System/Components/AC_GameplayTags.GetActiveTagContainer` (`self.GetComponentByClass` (`self.TargetUnit`) "/Game/Game/System/Components/AC_GameplayTags.AC_GameplayTags_C")))
  (return (and (`BlueprintGameplayTagLibrary.HasAllTags` _tagcontainer (`self.RequiredTags`)) (not (`BlueprintGameplayTagLibrary.HasAnyTags` _tagcontainer (`self.PreventingTags`) true)))))

(fn `UserConstructionScript`)