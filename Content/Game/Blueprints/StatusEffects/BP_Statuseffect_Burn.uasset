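; BP_Statuseffect_Burn is a burn status effect that damages the actor it is attached to.
; On each IntervalEffect event it requires the Instigator to be a BP_Unit, then calls ApplyDamage on the parent actor with the Instigator as damage causer.
; Damage amount and type are not yet set; an unconnected draft loop over the unit's weapon attribute modifiers notes the intent to derive them from the weapon or action.
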(event `self.IntervalEffect`
  (bind _instigator (`self.Instigator`))
  (bind _asbp_unit (cast `/Game/Game/Blueprints/Units/BP_Unit` _instigator))
  (`GameplayStatics.ApplyDamage` (`self.GetParentActor`) 0.0 null _instigator))

(fn `UserConstructionScript`
  (`parent.UserConstructionScript`))