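; Networked ability actor for a turn-based game, placed by its owner and executed in a set phase.
; Until set, it follows the mouse, range-clamped and floor-traced; a click sends the location to the server, and RepNotifies update position and team visibility.
; Phase changes queue it on GS_TurnBased; execution turns the unit and spawns effect actors, signalling completion when all finish.
; A gated cooldown counts down on later phase changes, then destroys the actor.
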(event `self.ReceiveTick`
  (params (DeltaSeconds :type "Float (single-precision)"))
  (if (`self.CanBePlaced`)
    (`self.K2_SetActorLocation` (`self.GetClampedLocationAtFloor`))))

(event `self.ReceiveBeginPlay`
  (`self.SetVisibiltyByController`)
  (`KismetSystemLibrary.Delay` 0.2)
  (`/Engine/EditorBlueprintResources/ActorMacros.Switch Has Authority`
    (:`Authority`
      (bind _asgs_turn_based (cast `/Game/Game/System/Gameplay/GS_TurnBased` (`GameplayStatics.GetGameState`)))
      (add `/Game/Game/System/Gameplay/GS_TurnBased.OnPhaseChanged` _asgs_turn_based (`|CreateDelegate` :!event `OnPhaseChanged`))
      (`self.CLIENT_SetLocation`))))

(event `CLIENT_SetLocation`
  (if (`/Game/Game/Blueprints/Abilities/Data/PDA_Action.LocationSetByMouse` (`self.Data`))
    (`self.EnableInput` (`GameplayStatics.GetPlayerController` 0))))

(event `StartCooldown`
  (`/Engine/EditorBlueprintResources/StandardMacros.DoOnce` false
    (:`Completed`
      (set `self.CooldownRemaining` (`/Game/Game/Blueprints/Abilities/Data/PDA_Action.CooldownLength` (`self.Data`)))
      (goto _label :!via `Open`))))

(event `OnPhaseChanged`
  (params (Phase :type "/Game/Game/System/Enums/EPhase Enum" :default "NewEnumerator5"))
  (if (`|EnumEquality` Phase "NewEnumerator0")
    (`/Engine/EditorBlueprintResources/StandardMacros.Gate` true :!label _label
      (:`Exit`
        (bind _result (`/Engine/EditorBlueprintResources/StandardMacros.DecrementInt` (`self.CooldownRemaining`))
          (:`  `
            (`self.OnCooldown` self)
            (if (<= _result 0)
              (`self.K2_DestroyActor`))))))
    (else
      (set `self.IsHidden` true)
      (if (`self.CanExecute` Phase)
        (bind _asgs_turn_based (cast `/Game/Game/System/Gameplay/GS_TurnBased` (`GameplayStatics.GetGameState`)))
        (`/Game/Game/System/Gameplay/GS_TurnBased.AddAbilityToExecuteQueue` _asgs_turn_based self)))))

(event `EnhancedInput|/Game/Game/System/Inputs/IA_SingleClick`
  (params (ActionValue :type Boolean) (ElapsedSeconds :type "Float (double-precision)") (TriggeredSeconds :type "Float (double-precision)") (InputAction :type "InputAction Object Reference" :default "/Game/Game/System/Inputs/IA_SingleClick.IA_SingleClick"))
  (:`Triggered`
    (`self.SERVER_SetLocation` (`self.GetMouseLocationInWorld`))
    (`self.DisableInput` (`GameplayStatics.GetPlayerController` 0))))

(event `SERVER_SetLocation`
  (params (NewLocation :type "Vector Structure"))
  (set `self.Location` NewLocation)
  (set `self.IsSet` true))

(event `OnExecute`
  (`self.TurnToTarget`)
  (`KismetSystemLibrary.Delay` 1.0)
  (`self.ExecuteEffects`))

(event `TurnToTarget`
  (bind _current_previewer (`self.Current Previewer`)
    (:`then`
      (`self.K2_SetActorRotation` (`self.Unit`) (`KismetMathLibrary.SelectRotator` (`KismetMathLibrary.Conv_VectorToRotator` (`KismetMathLibrary.GetDirectionUnitVector` (`self.K2_GetActorLocation`) (`self.K2_GetActorLocation` _current_previewer))) (`self.K2_GetActorRotation` _current_previewer) (`/Game/Game/Blueprints/Abilities/Data/PDA_Action.LocationSetByMouse` (`self.Data`))) false))
    (:`else`)))

(fn `CanBePlaced`
  (returns (ReturnValue :type Boolean))
  (return (and (not (`self.IsSet`)) (== (`self.GetOwner`) (`GameplayStatics.GetPlayerController` 0)))))

(fn `CanExecute`
  (params (Phase :type "/Game/Game/System/Enums/EPhase Enum" :default "NewEnumerator5"))
  (returns (ReturnValue :type Boolean))
  (return (`|EnumEquality` Phase (`/Game/Game/Blueprints/Abilities/Data/PDA_Action.ExecutionPhase` (`self.Data`)))))

(fn `ExecuteEffects`
  (for (_array_element _array_index) (`self.Effects`)
    (bind _returnvalue (`|SpawnActorFromClass` _array_element (`self.GetTransform`) "AlwaysSpawn" "MultiplyWithRoot" null (`self.Unit`) null))
    (`KismetArrayLibrary.Array_Remove` (`self.Effects`) _array_index)
    (`KismetArrayLibrary.Array_AddUnique` (`self.SpawnedEffects`) _returnvalue)
    (add `/Game/Game/Blueprints/Abilities/BP_Effect.OnEffectCompleted` _returnvalue (`|CreateDelegate` :!event `Is Ability Finished`)))
  (`self.StartCooldown`))

(fn `GetAbilityName`
  (returns (Name :type Text))
  (return (`/Game/Game/Blueprints/Abilities/Data/PDA_Action.Name` (`self.Data`))))

(fn `GetClampedLocation`
  (params (Range :type "Float (double-precision)"))
  (returns (ReturnValue :type "Vector Structure"))
  (return (+ (* (`self.GetDirectionToMouse`) Range) (`self.K2_GetActorLocation` (`self.Unit`)))))

(fn `GetClampedLocationAtFloor`
  (returns (Location :type "Vector Structure"))
  (bind _placementrange (`self.GetPlacementRange`))
  (bind _returnvalue (`KismetMathLibrary.SelectVector` (`self.GetClampedLocation` _placementrange) (`self.GetMouseLocationInWorld`) (> (`self.GetDistanceToMouse`) _placementrange)))
  (bind _outhit (`KismetSystemLibrary.LineTraceSingle` :`Start` (+ _returnvalue (0.0 0.0 300.0)) :`End` (- _returnvalue (0.0 0.0 300.0)) :`TraceChannel` "TraceTypeQuery1" :`DrawDebugType` "ForOneFrame"))
  (return (`.Location` (`GameplayStatics.BreakHitResult` _outhit))))

(fn `GetDirectionToMouse`
  (returns (ReturnValue :type "Vector Structure"))
  (return (`KismetMathLibrary.GetDirectionUnitVector` (`self.K2_GetActorLocation` (`self.Unit`)) (`self.GetMouseLocationInWorld`))))

(fn `GetDistanceToMouse`
  (returns (ReturnValue :type "Float (double-precision)"))
  (return (`KismetMathLibrary.Vector_Distance` (`self.GetMouseLocationInWorld`) (`self.K2_GetActorLocation` (`self.Unit`)))))

(fn `GetMouseLocationInWorld`
  (returns (Location :type "Vector Structure"))
  (return (`.Location` (`GameplayStatics.BreakHitResult` (`PlayerController.GetHitResultUnderCursorByChannel` (`GameplayStatics.GetPlayerController` 0) "TraceTypeQuery1" true)))))

(fn `GetPlacementRange`
  (returns (PlacementRange :type "Float (double-precision)"))
  (bind _returnvalue (`/Game/Game/Blueprints/Abilities/Data/PDA_Action.GetUnitModifiedRange` (`self.Data`) (`self.Unit`)))
  (return _returnvalue))

(fn `Is Ability Finished`
  (params (Effect :type "/Game/Game/Blueprints/Abilities/BP_Effect Object Reference"))
  (bind _spawnedeffects (`self.SpawnedEffects`))
  (`KismetArrayLibrary.Array_RemoveItem` _spawnedeffects Effect)
  (if (`KismetArrayLibrary.Array_IsEmpty` _spawnedeffects)
    (`self.OnAbilityComplete`)))

(fn `OnRep_IsHidden`
  (`self.SetActorHiddenInGame` (`self.IsHidden`)))

(fn `OnRep_IsSet`
  (if (`self.IsSet`)
    (`self.SetVisibilityByTeam`)
    (bind _aspc_turn_based (cast `/Game/Game/System/Gameplay/PC_TurnBased` (`GameplayStatics.GetPlayerController` 0)))
    (`/Game/Game/System/Gameplay/PC_TurnBased.OnAbilityCreated` _aspc_turn_based)))

(fn `OnRep_Location`
  (`self.K2_SetActorLocation` (`self.Location`)))

(fn `SetVisibilityByTeam`
  (bind _aspc_turn_based (cast `/Game/Game/System/Gameplay/PC_TurnBased` (`GameplayStatics.GetPlayerController` 0)))
  (`self.SetActorHiddenInGame` (not (`|EnumEquality` (`/Game/Game/System/Components/AC_Attributes.Team` (`/Game/Game/Blueprints/Units/BP_Unit.AC_Attributes` (`self.Unit`))) (`/Game/Game/System/Components/AC_Attributes.Team` (`/Game/Game/Blueprints/Units/BP_Unit.AC_Attributes` (`/Game/Game/System/Gameplay/PC_TurnBased.CurrentUnit` _aspc_turn_based)))))))

(fn `SetVisibiltyByController`
  (bind _aspc_turn_based (cast `/Game/Game/System/Gameplay/PC_TurnBased` (`GameplayStatics.GetPlayerController` 0)))
  (`self.SetActorHiddenInGame` (not (== (`/Game/Game/System/Gameplay/PC_TurnBased.CurrentUnit` _aspc_turn_based) (`self.Unit`)))))

(fn `UserConstructionScript`)