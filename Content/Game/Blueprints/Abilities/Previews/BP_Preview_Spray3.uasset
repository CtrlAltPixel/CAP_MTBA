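; Ability preview actor that shows a three-lane spray aimed at the point under the player's cursor.
; Each tick it scales three decals from the ability's radius and placement range, then fans them around the aim yaw by the ability's angle.
; It runs a debug-drawn box trace along each lane and tints all three decals red when any hits, white otherwise.
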(event `self.ReceiveTick`
  (params (DeltaSeconds :type "Float (single-precision)"))
  (bind _abilitydata (`self.AbilityData`))
  (bind _abilitydata_2 (`self.AbilityData`))
  (bind _angle (`/Game/Game/Blueprints/Abilities/Data/DA_Action.Angle` (`self.AbilityData`)))
  (bind _radius (`/Game/Game/Blueprints/Abilities/Data/DA_Action.Radius` (`self.AbilityData`)))
  (`parent.ReceiveTick` DeltaSeconds)
  (`SceneComponent.SetWorldScale3D` (`self.Scene`) (`KismetMathLibrary.MakeVector` 1.0 (/ (`/Game/Game/Blueprints/Abilities/Data/DA_Action.Radius` _abilitydata_2) 100.0) (/ (`/Game/Game/Blueprints/Abilities/Data/DA_Action.PlacementRange` _abilitydata_2) 200.0)))
  (`SceneComponent.SetWorldScale3D` (`self.Scene1`) (`KismetMathLibrary.MakeVector` 1.0 (/ (`/Game/Game/Blueprints/Abilities/Data/DA_Action.Radius` _abilitydata_2) 100.0) (/ (`/Game/Game/Blueprints/Abilities/Data/DA_Action.PlacementRange` _abilitydata_2) 200.0)))
  (`SceneComponent.SetWorldScale3D` (`self.Scene2`) (`KismetMathLibrary.MakeVector` 1.0 (/ (`/Game/Game/Blueprints/Abilities/Data/DA_Action.Radius` _abilitydata_2) 100.0) (/ (`/Game/Game/Blueprints/Abilities/Data/DA_Action.PlacementRange` _abilitydata_2) 200.0)))
  (`self.RotateDecal`)
  (set `self.HasTarget` false)
  (for _index (range 3)
    (bind _returnvalue (`KismetMathLibrary.ComposeRotators` (`KismetMathLibrary.ComposeRotators` (`self.AimDirection`) (`KismetMathLibrary.MakeRotator` 0.0 0.0 (* _index _angle))) (`KismetMathLibrary.MakeRotator` 0.0 0.0 (+ (/ (* _angle 3.0) -2.0) (/ _angle 2.0)))))
    (bind (_outhit _returnvalue_2) (`KismetSystemLibrary.BoxTraceSingle` :`Start` (+ (`self.K2_GetActorLocation`) (* (`KismetMathLibrary.GetForwardVector` (`self.AimDirection`)) (`/Game/Game/Blueprints/Abilities/Data/DA_Action.Radius` (`self.AbilityData`)))) :`End` (+ (`self.K2_GetActorLocation`) (* (`KismetMathLibrary.GetForwardVector` _returnvalue) (- (`/Game/Game/Blueprints/Abilities/Data/DA_Action.PlacementRange` _abilitydata) (`/Game/Game/Blueprints/Abilities/Data/DA_Action.Radius` _abilitydata)))) :`HalfSize` (`KismetMathLibrary.MakeVector` _radius _radius 50.0) :`Orientation` _returnvalue :`TraceChannel` "TraceTypeQuery3" :`DrawDebugType` "ForOneFrame"))
    (if _returnvalue_2
      (set `self.HasTarget` true)))
  (`DecalComponent.SetDecalColor` (`self.Decal`) (`KismetMathLibrary.SelectColor` (struct :`R` 1.0 :`A` 1.0) (struct :`R` 1.0 :`G` 1.0 :`B` 1.0 :`A` 1.0) (`self.HasTarget`)))
  (`DecalComponent.SetDecalColor` (`self.Decal1`) (`KismetMathLibrary.SelectColor` (struct :`R` 1.0 :`A` 1.0) (struct :`R` 1.0 :`G` 1.0 :`B` 1.0 :`A` 1.0) (`self.HasTarget`)))
  (`DecalComponent.SetDecalColor` (`self.Decal2`) (`KismetMathLibrary.SelectColor` (struct :`R` 1.0 :`A` 1.0) (struct :`R` 1.0 :`G` 1.0 :`B` 1.0 :`A` 1.0) (`self.HasTarget`))))

(fn `RotateDecal`
  (bind (_returnvalue_roll _returnvalue_pitch _returnvalue_yaw) (`KismetMathLibrary.BreakRotator` (`KismetMathLibrary.FindLookAtRotation` (`self.K2_GetActorLocation`) (`.Location` (`GameplayStatics.BreakHitResult` (`PlayerController.GetHitResultUnderCursorByChannel` (`GameplayStatics.GetPlayerController` 0) "TraceTypeQuery1" true))))))
  (bind _output_get (set `self.AimDirection` (`KismetMathLibrary.MakeRotator` 0.0 0.0 _returnvalue_yaw)))
  (`SceneComponent.K2_SetWorldRotation` (`self.Scene`) (`KismetMathLibrary.MakeRotator` 0.0 -90.0 (- (.yaw _output_get) (`/Game/Game/Blueprints/Abilities/Data/DA_Action.Angle` (`self.AbilityData`)))) false false)
  (`SceneComponent.K2_SetWorldRotation` (`self.Scene1`) (`KismetMathLibrary.MakeRotator` 0.0 -90.0 (.yaw _output_get)) false false)
  (`SceneComponent.K2_SetWorldRotation` (`self.Scene2`) (`KismetMathLibrary.MakeRotator` 0.0 -90.0 (+ (.yaw _output_get) (`/Game/Game/Blueprints/Abilities/Data/DA_Action.Angle` (`self.AbilityData`)))) false false))

(fn `UserConstructionScript`
  (`parent.UserConstructionScript`))