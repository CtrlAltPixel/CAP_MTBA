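; Box-shaped ability placement preview that aims a decal from the actor toward the world point under the cursor, using yaw only.
; Each tick it scales the decal from the ability's radius and placement range, rotates it and clears HasTarget.
; A debug-drawn box trace along the aim axis, extending both behind and ahead of the actor, turns the decal red on a hit and white otherwise.
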(event `self.ReceiveTick`
  (params (DeltaSeconds :type "Float (single-precision)"))
  (bind _returnvalue (`self.K2_GetActorLocation`))
  (bind _abilitydata (`self.AbilityData`))
  (bind _abilitydata_2 (`self.AbilityData`))
  (bind _radius (`/Game/Game/Blueprints/Abilities/Data/DA_Action.Radius` (`self.AbilityData`)))
  (bind _returnvalue_2 (* (`KismetMathLibrary.GetForwardVector` (`self.AimDirection`)) (- (`/Game/Game/Blueprints/Abilities/Data/DA_Action.PlacementRange` _abilitydata) (`/Game/Game/Blueprints/Abilities/Data/DA_Action.Radius` _abilitydata))))
  (`parent.ReceiveTick` DeltaSeconds)
  (`SceneComponent.SetWorldScale3D` (`self.Decal`) (`KismetMathLibrary.MakeVector` 1.0 (/ (`/Game/Game/Blueprints/Abilities/Data/DA_Action.Radius` _abilitydata_2) 200.0) (/ (`/Game/Game/Blueprints/Abilities/Data/DA_Action.PlacementRange` _abilitydata_2) 200.0)))
  (`self.RotateDecal`)
  (set `self.HasTarget` false)
  (bind (_outhit _returnvalue_3) (`KismetSystemLibrary.BoxTraceSingle` :`Start` (- _returnvalue _returnvalue_2) :`End` (+ _returnvalue _returnvalue_2) :`HalfSize` (`KismetMathLibrary.MakeVector` _radius _radius) :`Orientation` (`self.AimDirection`) :`TraceChannel` "TraceTypeQuery3" :`DrawDebugType` "ForOneFrame"))
  (`DecalComponent.SetDecalColor` (`self.Decal`) (`KismetMathLibrary.SelectColor` (struct :`R` 1.0 :`A` 1.0) (struct :`R` 1.0 :`G` 1.0 :`B` 1.0 :`A` 1.0) _returnvalue_3)))

(fn `RotateDecal`
  (bind (_returnvalue_roll _returnvalue_pitch _returnvalue_yaw) (`KismetMathLibrary.BreakRotator` (`KismetMathLibrary.FindLookAtRotation` (`self.K2_GetActorLocation`) (`.Location` (`GameplayStatics.BreakHitResult` (`PlayerController.GetHitResultUnderCursorByChannel` (`GameplayStatics.GetPlayerController` 0) "TraceTypeQuery1" true))))))
  (bind _output_get (set `self.AimDirection` (`KismetMathLibrary.MakeRotator` 0.0 0.0 _returnvalue_yaw)))
  (`SceneComponent.K2_SetWorldRotation` (`self.Decal`) (`KismetMathLibrary.MakeRotator` 0.0 -90.0 (.yaw _output_get)) false false))

(fn `UserConstructionScript`
  (`parent.UserConstructionScript`))