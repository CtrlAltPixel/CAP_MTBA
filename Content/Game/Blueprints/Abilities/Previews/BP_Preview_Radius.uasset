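; Ability preview that shows a cursor-aimed decal and colors it red when its traces hit something, white otherwise.
; While previewing, each tick scales the decal by the unit's modified range and yaws the actor toward the cursor hit point.
; It then sweeps a fan of debug-drawn line traces from the unit's floor point, using the ability's angle and unmodified placement range.
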(event `self.ReceiveTick`
  (params (DeltaSeconds :type "Float (single-precision)"))
  (bind _unit (`self.Unit`))
  (bind (_floorresult_bblockinghit _floorresult_bwalkablefloor _floorresult_blinetrace _floorresult_floordist _floorresult_linedist _floorresult_hitresult) (break `FindFloorResult` (`CharacterMovementComponent.K2_FindFloor` (`Character.CharacterMovement` _unit) (`self.K2_GetActorLocation` _unit))))
  (bind (_bblockinghit _binitialoverlap _time _distance _location) (`GameplayStatics.BreakHitResult` _floorresult_hitresult))
  (`parent.ReceiveTick` DeltaSeconds)
  (if (`self.IsPreviewing`)
    (`self.AdjustDecal`)
    (set `self.HasTarget` false)
    (for _index (range (+ (`KismetMathLibrary.FTrunc` (* (/ (`/Game/Game/Blueprints/Abilities/Data/DA_Action.Angle` (`self.AbilityData`)) 5.0) 2.0)) 1))
      (bind (_outhit _returnvalue) (`KismetSystemLibrary.LineTraceSingle` _location (+ _location (* (`KismetMathLibrary.GreaterGreater_VectorRotator` (`KismetMathLibrary.GetForwardVector` (`self.AimDirection`)) (`KismetMathLibrary.MakeRotator` 0.0 0.0 (- (* _index 2.0) (/ (`/Game/Game/Blueprints/Abilities/Data/DA_Action.Angle` (`self.AbilityData`)) 2.0)))) (`/Game/Game/Blueprints/Abilities/Data/DA_Action.PlacementRange` (`self.AbilityData`)))) "TraceTypeQuery3" false (`|MakeArray` (`self.Unit`) :!type "Actor Object Reference") "ForOneFrame"))
      (if _returnvalue
        (set `self.HasTarget` true)))
    (`DecalComponent.SetDecalColor` (`self.Decal`) (`KismetMathLibrary.SelectColor` (struct :`R` 1.0 :`A` 1.0) (struct :`R` 1.0 :`G` 1.0 :`B` 1.0 :`A` 1.0) (`self.HasTarget`)))))

(fn `AdjustDecal`
  (bind _abilitydata (`self.AbilityData`)
    (:`then`
      (bind _returnvalue (`/Game/Game/Blueprints/Abilities/Data/DA_Action.GetUnitModifiedRange` _abilitydata (`self.Unit`)))
      (`SceneComponent.SetWorldScale3D` (`self.Decal`) (`KismetMathLibrary.Conv_DoubleToVector` (/ _returnvalue 100.0)))
      (`self.RotateDecal`))
    (:`else`)))

(fn `RotateDecal`
  (bind (_returnvalue_roll _returnvalue_pitch _returnvalue_yaw) (`KismetMathLibrary.BreakRotator` (`KismetMathLibrary.FindLookAtRotation` (`self.K2_GetActorLocation`) (`.Location` (`GameplayStatics.BreakHitResult` (`PlayerController.GetHitResultUnderCursorByChannel` (`GameplayStatics.GetPlayerController` 0) "TraceTypeQuery1" true))))))
  (bind _output_get (set `self.AimDirection` (`KismetMathLibrary.MakeRotator` 0.0 0.0 _returnvalue_yaw)))
  (`self.K2_SetActorRotation` (`KismetMathLibrary.MakeRotator` 0.0 0.0 (.yaw _output_get))))

(fn `UserConstructionScript`
  (`parent.UserConstructionScript`))