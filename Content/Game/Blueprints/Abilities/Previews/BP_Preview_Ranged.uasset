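; Ranged ability preview actor that shows the area of effect at the cursor while the player aims.
; On BeginPlay it scales its decal from the ability's radius.
; While previewing, Tick follows the visibility trace under the cursor within placement range of the unit, otherwise holding the last in-range point.
; Sphere overlaps toggle highlighting on units entering or leaving the area.
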(event `self.ReceiveBeginPlay`
  (`parent.ReceiveBeginPlay`)
  (`SceneComponent.SetWorldScale3D` (`self.Decal`) (/ (`/Game/Game/Blueprints/Abilities/Data/PDA_Action.Radius` (`self.AbilityData`)) 100.0)))

(event `self.ReceiveTick`
  (params (DeltaSeconds :type "Float (single-precision)"))
  (bind _hitresult (`PlayerController.GetHitResultUnderCursorByChannel` (`GameplayStatics.GetPlayerController` 0) "TraceTypeQuery1" true))
  (`parent.ReceiveTick` DeltaSeconds)
  (if (`self.IsPreviewing`)
    (if (<= (`KismetMathLibrary.Vector_Distance` (`.Location` (`GameplayStatics.BreakHitResult` _hitresult)) (`self.K2_GetActorLocation` (`self.Unit`))) (`/Game/Game/Blueprints/Abilities/Data/PDA_Action.PlacementRange` (`self.AbilityData`)))
      (bind _output_get (set `self.Hit Result Location` (`.Location` (`GameplayStatics.BreakHitResult` _hitresult))))
      (`self.K2_SetActorLocation` _output_get)
      (else
        (`self.K2_SetActorLocation` (`self.Hit Result Location`))))))

(event `self.Sphere.OnComponentBeginOverlap`
  (params (OverlappedComponent :type "PrimitiveComponent Object Reference") (OtherActor :type "Actor Object Reference") (OtherComp :type "PrimitiveComponent Object Reference") (OtherBodyIndex :type Integer) (bFromSweep :type Boolean) (SweepResult :type "HitResult Structure (by ref)"))
  (bind _asbp_unit (cast `/Game/Game/Blueprints/Units/BP_Unit` OtherActor))
  (`/Game/Game/Blueprints/Units/BP_Unit.HighlightUnit` _asbp_unit true))

(event `self.Sphere.OnComponentEndOverlap`
  (params (OverlappedComponent :type "PrimitiveComponent Object Reference") (OtherActor :type "Actor Object Reference") (OtherComp :type "PrimitiveComponent Object Reference") (OtherBodyIndex :type Integer))
  (bind _asbp_unit (cast `/Game/Game/Blueprints/Units/BP_Unit` OtherActor))
  (`/Game/Game/Blueprints/Units/BP_Unit.HighlightUnit` _asbp_unit false))

(fn `UserConstructionScript`
  (`parent.UserConstructionScript`))