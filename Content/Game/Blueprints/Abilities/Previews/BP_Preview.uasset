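; Preview actor for placing a unit's ability in a turn-based game, registered on the server as the PlayerController's CurrentPreviewer.
; Confirming the preview checks the Unit's resource against the ability cost, locks rotation through an MC_SetRotation event and deducts the cost; cancelling refunds it and destroys the actor.
; Game state phase changes hide it during Spells and destroy it at Respawn.
; A PlayerState-based resource path exists but is unwired.
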(event `self.ReceiveTick`
  (params (DeltaSeconds :type "Float (single-precision)")))

(event `self.ReceiveBeginPlay`
  (`/Engine/EditorBlueprintResources/ActorMacros.Switch Has Authority`
    (:`Authority`
      (set `/Game/Game/System/Gameplay/PC_TurnBased.CurrentPreviewer` self (`self.PlayerController`))
      (bind _asgs_turn_based (cast `/Game/Game/System/Gameplay/GS_TurnBased` (`GameplayStatics.GetGameState`)))
      (add `/Game/Game/System/Gameplay/GS_TurnBased.OnPhaseChanged` _asgs_turn_based (`|CreateDelegate` :!event `OnPhaseChanged`)))))

(event `OnSetPreview`
  (params (NewRotation :type "Rotator Structure"))
  (bind _ac_attributes (`/Game/Game/Blueprints/Units/BP_Unit.AC_Attributes` (`self.Unit`)))
  (if (`self.CanCastAbility`)
    (`self.MC_SetRotation` NewRotation)
    (set `self.IsPreviewing` false)
    ;[1 0 0] Swap with Player State Version? (Also needs on Cancel)
    (set `/Game/Game/System/Components/AC_Attributes.Resource` (- (`/Game/Game/System/Components/AC_Attributes.Resource` _ac_attributes) (`/Game/Game/Blueprints/Abilities/Data/PDA_Action.ResourceCost` (`self.AbilityData`))) _ac_attributes)
    (else
      (`KismetSystemLibrary.PrintString` "Not enough resource"))))

(event `MC_SetRotation`
  (params (NewRotation :type "Rotator Structure"))
  (`self.K2_SetActorRotation` NewRotation)
  (set `self.IsPreviewing` false))

(event `OnPhaseChanged`
  (params (Phase :type "/Game/Game/System/Enums/EPhase Enum" :default "NewEnumerator5"))
  (switch `/Game/Game/System/Enums/EPhase` Phase
    (:`NewEnumerator7`
      (`self.SetActorHiddenInGame` true))
    (:`NewEnumerator8`
      (`self.K2_DestroyActor`))))

(event `Cancelled`
  (bind _ac_attributes (`/Game/Game/Blueprints/Units/BP_Unit.AC_Attributes` (`self.Unit`)))
  (set `/Game/Game/System/Components/AC_Attributes.Resource` (+ (`/Game/Game/System/Components/AC_Attributes.Resource` _ac_attributes) (`/Game/Game/Blueprints/Abilities/Data/PDA_Action.ResourceCost` (`self.AbilityData`))) _ac_attributes)
  (`self.K2_DestroyActor`))

(fn `CanCastAbility`
  (returns (ReturnValue :type Boolean))
  (return (>= (`/Game/Game/System/Components/AC_Attributes.Resource` (`/Game/Game/Blueprints/Units/BP_Unit.AC_Attributes` (`self.Unit`))) (`/Game/Game/Blueprints/Abilities/Data/PDA_Action.ResourceCost` (`self.AbilityData`)))))

(fn `SetPreview`
  (set `self.IsPreviewing` false))

(fn `UserConstructionScript`)