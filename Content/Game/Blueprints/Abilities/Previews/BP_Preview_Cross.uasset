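; Ability placement preview that shows a cross-shaped area centered on the actor and turned toward the cursor.
; Each tick, it scales two perpendicular decals from the ability's radius and placement range, then yaws them to face the point under the cursor.
; Box traces along both arms turn the decals red on a hit and white otherwise, with per-frame debug drawing left on.
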(event `self.ReceiveTick`
  (params (DeltaSeconds :type "Float (single-precision)"))
  (bind _returnvalue (`self.K2_GetActorLocation`))
  (bind _returnvalue_2 (`self.K2_GetActorLocation`))
  (bind _abilitydata (`self.AbilityData`))
  (bind _abilitydata_2 (`self.AbilityData`))
  (bind _abilitydata_3 (`self.AbilityData`))
  (bind _radius (`/Game/Game/Blueprints/Abilities/Data/DA_Ability.Radius` (`self.AbilityData`)))
  (bind _returnvalue_3 (`KismetMathLibrary.MakeVector` _radius _radius))
  (bind _returnvalue_4 (* (`KismetMathLibrary.GetRightVector` (`self.AimDirection`)) (- (`/Game/Game/Blueprints/Abilities/Data/DA_Ability.PlacementRange` _abilitydata) (`/Game/Game/Blueprints/Abilities/Data/DA_Ability.Radius` _abilitydata))))
  (bind _returnvalue_5 (* (`KismetMathLibrary.GetForwardVector` (`self.AimDirection`)) (- (`/Game/Game/Blueprints/Abilities/Data/DA_Ability.PlacementRange` _abilitydata_2) (`/Game/Game/Blueprints/Abilities/Data/DA_Ability.Radius` _abilitydata_2))))
  (`parent.ReceiveTick` DeltaSeconds)
  (`SceneComponent.SetWorldScale3D` (`self.Decal`) (`KismetMathLibrary.MakeVector` 1.0 (/ (`/Game/Game/Blueprints/Abilities/Data/DA_Ability.Radius` _abilitydata_3) 200.0) (/ (`/Game/Game/Blueprints/Abilities/Data/DA_Ability.PlacementRange` _abilitydata_3) 200.0)))
  (`SceneComponent.SetWorldScale3D` (`self.Decal1`) (`KismetMathLibrary.MakeVector` 1.0 (/ (`/Game/Game/Blueprints/Abilities/Data/DA_Ability.Radius` _abilitydata_3) 200.0) (/ (`/Game/Game/Blueprints/Abilities/Data/DA_Ability.PlacementRange` _abilitydata_3) 200.0)))
  (`self.RotateDecal`)
  (set `self.HasTarget` false)
  (bind (_outhit _returnvalue_6) (`KismetSystemLibrary.BoxTraceSingle` :`Start` (- _returnvalue _returnvalue_5) :`End` (+ _returnvalue _returnvalue_5) :`HalfSize` _returnvalue_3 :`Orientation` (`self.AimDirection`) :`TraceChannel` "TraceTypeQuery3" :`DrawDebugType` "ForOneFrame"))
  (if _returnvalue_6
    (set `self.HasTarget` true))
  (bind (_outhit_2 _returnvalue_7) (`KismetSystemLibrary.BoxTraceSingle` :`Start` (- _returnvalue_2 _returnvalue_4) :`End` (+ _returnvalue_2 _returnvalue_4) :`HalfSize` _returnvalue_3 :`Orientation` (`KismetMathLibrary.ComposeRotators` (`self.AimDirection`) (struct :`Yaw` 90.0)) :`TraceChannel` "TraceTypeQuery3" :`DrawDebugType` "ForOneFrame"))
  (`DecalComponent.SetDecalColor` (`self.Decal`) (`KismetMathLibrary.SelectColor` (struct :`R` 1.0 :`A` 1.0) (struct :`R` 1.0 :`G` 1.0 :`B` 1.0 :`A` 1.0) (or _returnvalue_7 (`self.HasTarget`))))
  (`DecalComponent.SetDecalColor` (`self.Decal1`) (`KismetMathLibrary.SelectColor` (struct :`R` 1.0 :`A` 1.0) (struct :`R` 1.0 :`G` 1.0 :`B` 1.0 :`A` 1.0) (or _returnvalue_7 (`self.HasTarget`)))))

(fn `RotateDecal`
  (bind (_returnvalue_roll _returnvalue_pitch _returnvalue_yaw) (`KismetMathLibrary.BreakRotator` (`KismetMathLibrary.FindLookAtRotation` (`self.K2_GetActorLocation`) (`.Location` (`GameplayStatics.BreakHitResult` (`PlayerController.GetHitResultUnderCursorByChannel` (`GameplayStatics.GetPlayerController` 0) "TraceTypeQuery1" true))))))
  (bind _output_get (set `self.AimDirection` (`KismetMathLibrary.MakeRotator` 0.0 0.0 _returnvalue_yaw)))
  (`SceneComponent.K2_SetWorldRotation` (`self.Decal`) (`KismetMathLibrary.MakeRotator` 0.0 -90.0 (.yaw _output_get)) false false)
  (`SceneComponent.K2_SetWorldRotation` (`self.Decal1`) (`KismetMathLibrary.MakeRotator` 0.0 -90.0 (+ (.yaw _output_get) 90.0)) false false))

(fn `UserConstructionScript`
  (`parent.UserConstructionScript`))