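; Ability preview actor that shows a line decal aimed from the actor toward the cursor while previewing.
; Each tick it scales the decal from the ability's radius and placement range, then yaws it toward the cursor's hit point.
; A box trace along that line, drawn for debug, tints the decal red on a hit, otherwise white.
; Despite the name, the reflection vector calculation is unused.
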(event `self.ReceiveTick`
  (params (DeltaSeconds :type "Float (single-precision)"))
  (bind _returnvalue (`self.K2_GetActorLocation`))
  (bind _abilitydata (`self.AbilityData`))
  (bind _abilitydata_2 (`self.AbilityData`))
  (bind _radius (`/Game/Game/Blueprints/Abilities/Data/PDA_Action.Radius` (`self.AbilityData`)))
  (`parent.ReceiveTick` DeltaSeconds)
  (if (`self.IsPreviewing`)
    (`SceneComponent.SetWorldScale3D` (`self.Scene`) (`KismetMathLibrary.MakeVector` 1.0 (/ (`/Game/Game/Blueprints/Abilities/Data/PDA_Action.Radius` _abilitydata_2) 100.0) (/ (`/Game/Game/Blueprints/Abilities/Data/PDA_Action.PlacementRange` _abilitydata_2) 200.0)))
    (`self.RotateDecal`)
    (set `self.HasTarget` false)
    (bind (_outhit _returnvalue_2) (`KismetSystemLibrary.BoxTraceSingle` :`Start` (+ _returnvalue (* (`KismetMathLibrary.GetForwardVector` (`self.AimDirection`)) (`/Game/Game/Blueprints/Abilities/Data/PDA_Action.Radius` (`self.AbilityData`)))) :`End` (+ _returnvalue (* (`KismetMathLibrary.GetForwardVector` (`self.AimDirection`)) (- (`/Game/Game/Blueprints/Abilities/Data/PDA_Action.PlacementRange` _abilitydata) (`/Game/Game/Blueprints/Abilities/Data/PDA_Action.Radius` _abilitydata)))) :`HalfSize` (`KismetMathLibrary.MakeVector` _radius _radius 50.0) :`Orientation` (`self.AimDirection`) :`TraceChannel` "TraceTypeQuery3" :`DrawDebugType` "ForOneFrame"))
    (`DecalComponent.SetDecalColor` (`self.Decal`) (`KismetMathLibrary.SelectColor` (struct :`R` 1.0 :`A` 1.0) (struct :`R` 1.0 :`G` 1.0 :`B` 1.0 :`A` 1.0) _returnvalue_2))))

(fn `RotateDecal`
  (bind (_returnvalue_roll _returnvalue_pitch _returnvalue_yaw) (`KismetMathLibrary.BreakRotator` (`KismetMathLibrary.FindLookAtRotation` (`self.K2_GetActorLocation`) (`.Location` (`GameplayStatics.BreakHitResult` (`PlayerController.GetHitResultUnderCursorByChannel` (`GameplayStatics.GetPlayerController` 0) "TraceTypeQuery1" true))))))
  (bind _output_get (set `self.AimDirection` (`KismetMathLibrary.MakeRotator` 0.0 0.0 _returnvalue_yaw)))
  (`SceneComponent.K2_SetWorldRotation` (`self.Scene`) (`KismetMathLibrary.MakeRotator` 0.0 -90.0 (.yaw _output_get)) false false))

(fn `UserConstructionScript`
  (`parent.UserConstructionScript`))