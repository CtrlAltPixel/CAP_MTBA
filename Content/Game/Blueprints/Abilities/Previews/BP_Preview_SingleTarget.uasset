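; Ability preview for single-target abilities that highlights the targeted unit and points a decal at it.
; Each tick, a sphere sized to the placement range gathers other units and picks the one nearest the cursor hit.
; The chosen unit gets a selection overlay material, clearing the previous one, while the decal rotates and stretches toward it using the ability radius for width.
; An older box-trace decal tint remains unconnected.
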(event `self.ReceiveTick`
  (params (DeltaSeconds :type "Float (single-precision)"))
  (`parent.ReceiveTick` DeltaSeconds)
  (`self.RotateDecal`))

(fn `FindClosestTarget`
  (returns (Closest :type "Actor Object Reference"))
  (locals (Local_CurrentClosestDistance :type "Float (double-precision)") (Local_Closest :type "Actor Object Reference"))
  (`SphereComponent.SetSphereRadius` (`self.Sphere`) (`/Game/Game/Blueprints/Abilities/Data/PDA_Action.PlacementRange` (`self.AbilityData`)) true)
  (bind _output_get (set `self.Overlapping Actors` (`PrimitiveComponent.GetOverlappingActors` (`self.Sphere`) "/Game/Game/Blueprints/Units/BP_Unit.BP_Unit_C")))
  (`KismetArrayLibrary.Array_Remove` _output_get (`KismetArrayLibrary.Array_Find` _output_get (`self.Unit`)))
  (bind _output_get_2 (set `local.Local_Closest` (`.ReturnValue` (`GameplayStatics.FindNearestActor` (`.Location` (`GameplayStatics.BreakHitResult` (`PlayerController.GetHitResultUnderCursorByChannel` (`GameplayStatics.GetPlayerController` 0) "TraceTypeQuery1" true))) (`self.Overlapping Actors`)))))
  (if (!= (`self.CurrenTarget`) _output_get_2)
    (bind _asbp_unit (cast `/Game/Game/Blueprints/Units/BP_Unit` (`local.Local_Closest`)))
    (`MeshComponent.SetOverlayMaterial` (`Character.Mesh` _asbp_unit) "/Game/Game/Materials/M_SelectionOverlay.M_SelectionOverlay")
    (bind _asbp_unit_2 (cast `/Game/Game/Blueprints/Units/BP_Unit` (`self.CurrenTarget`))
      (:`then`
        (`MeshComponent.SetOverlayMaterial` (`Character.Mesh` _asbp_unit_2) null)
        (return (`local.Local_Closest`)))
      (:`CastFailed`
        (return (`local.Local_Closest`))))
    (else
      (return (`local.Local_Closest`)))))

(fn `RotateDecal`
  (bind _closest (`self.FindClosestTarget`))
  (`/Engine/EditorBlueprintResources/StandardMacros.IsValid` _closest
    (:`Is Valid`
      (set `self.CurrenTarget` _closest)
      (bind (_returnvalue_roll _returnvalue_pitch _returnvalue_yaw) (`KismetMathLibrary.BreakRotator` (`KismetMathLibrary.FindLookAtRotation` (`self.K2_GetActorLocation`) (`self.K2_GetActorLocation` _closest))))
      (bind _output_get (set `self.AimDirection` (`KismetMathLibrary.MakeRotator` 0.0 0.0 _returnvalue_yaw)))
      (`SceneComponent.K2_SetWorldRotation` (`self.Scene`) (`KismetMathLibrary.MakeRotator` 0.0 -90.0 (.yaw _output_get)) false false)
      (`self.CurrenTarget`
        (:`then`
          (`SceneComponent.SetWorldScale3D` (`self.Scene`) (`KismetMathLibrary.MakeVector` 1.0 (/ (`/Game/Game/Blueprints/Abilities/Data/PDA_Action.Radius` (`self.AbilityData`)) 100.0) (/ (`KismetMathLibrary.Vector_Distance` (`self.K2_GetActorLocation` (`self.CurrenTarget`)) (`self.K2_GetActorLocation`)) 200.0))))
        (:`else`
          (`SceneComponent.SetWorldScale3D` (`self.Scene`) (1.0 0.0 0.0)))))))

(fn `UserConstructionScript`
  (`parent.UserConstructionScript`))