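; Ability targeting preview that shows a fixed-size quad decal at the cursor, sized from the ability's Radius and Angle data.
; Each tick it follows the visibility trace under the cursor, holding the last stored location when the cursor leaves placement range of the casting unit.
; Its yaw follows the direction from that unit to the cursor.
; Box overlaps toggle highlighting on units inside the area.
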(event `self.ReceiveBeginPlay`
  (bind _abilitydata (`self.AbilityData`))
  (`parent.ReceiveBeginPlay`)
  (`SceneComponent.SetWorldScale3D` (`self.Decal`) (`KismetMathLibrary.MakeVector` 1.0 (/ (`/Game/Game/Blueprints/Abilities/Data/DA_Action.Radius` _abilitydata) 200.0) (/ (`/Game/Game/Blueprints/Abilities/Data/DA_Action.Angle` _abilitydata) 100.0))))

(event `self.ReceiveTick`
  (params (DeltaSeconds :type "Float (single-precision)"))
  (`parent.ReceiveTick` DeltaSeconds)
  (`self.SetPosition`)
  (`self.SetRotation`))

(event `self.Box.OnComponentBeginOverlap`
  (params (OverlappedComponent :type "PrimitiveComponent Object Reference") (OtherActor :type "Actor Object Reference") (OtherComp :type "PrimitiveComponent Object Reference") (OtherBodyIndex :type Integer) (bFromSweep :type Boolean) (SweepResult :type "HitResult Structure (by ref)"))
  (bind _asbp_unit (cast `/Game/Game/Blueprints/Units/BP_Unit` OtherActor))
  (`/Game/Game/Blueprints/Units/BP_Unit.HighlightUnit` _asbp_unit true))

(event `self.Box.OnComponentEndOverlap`
  (params (OverlappedComponent :type "PrimitiveComponent Object Reference") (OtherActor :type "Actor Object Reference") (OtherComp :type "PrimitiveComponent Object Reference") (OtherBodyIndex :type Integer))
  (bind _asbp_unit (cast `/Game/Game/Blueprints/Units/BP_Unit` OtherActor))
  (`/Game/Game/Blueprints/Units/BP_Unit.HighlightUnit` _asbp_unit false))

(fn `SetPosition`
  (bind _hitresult (`PlayerController.GetHitResultUnderCursorByChannel` (`GameplayStatics.GetPlayerController` 0) "TraceTypeQuery1" true))
  (if (<= (`KismetMathLibrary.Vector_Distance` (`.Location` (`GameplayStatics.BreakHitResult` _hitresult)) (`self.K2_GetActorLocation` (`self.Unit`))) (`/Game/Game/Blueprints/Abilities/Data/DA_Action.PlacementRange` (`self.AbilityData`)))
    (bind _output_get (set `self.Hit Result Location` (`.Location` (`GameplayStatics.BreakHitResult` _hitresult))))
    (`self.K2_SetActorLocation` _output_get)
    (else
      (`self.K2_SetActorLocation` (`self.Hit Result Location`)))))

(fn `SetRotation`
  (bind (_returnvalue_roll _returnvalue_pitch _returnvalue_yaw) (`KismetMathLibrary.BreakRotator` (`KismetMathLibrary.Conv_VectorToRotator` (`KismetMathLibrary.GetDirectionUnitVector` (`self.K2_GetActorLocation` (`self.Unit`)) (`.Location` (`GameplayStatics.BreakHitResult` (`PlayerController.GetHitResultUnderCursorByChannel` (`GameplayStatics.GetPlayerController` 0) "TraceTypeQuery1" true)))))))
  (`self.K2_SetActorRotation` (`KismetMathLibrary.MakeRotator` 0.0 0.0 _returnvalue_yaw)))

(fn `UserConstructionScript`
  (`parent.UserConstructionScript`))