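; BP_UltimateAnimation plays a Unit's ultimate ability cinematic from a given Level Sequence.
; On BeginPlay it creates a sequence player that disables movement input and hides the HUD.
; It overrides the transform origin to the Unit's location with zero rotation, so the sequence plays where the Unit stands.
; The Unit replaces the actor bound under the "Unit" tag before playback starts.
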(event `self.ReceiveBeginPlay`
  (bind (_outactor _returnvalue) (`LevelSequencePlayer.CreateLevelSequencePlayer` (`self.UltimateSequence`) (make `MovieSceneSequencePlaybackSettings` false (struct) 1.0 0.0 false false true false false true)))
  (set `LevelSequenceActor.bOverrideInstanceData` true _outactor)
  (bind _asdefault_level_sequence_instance_data (cast `DefaultLevelSequenceInstanceData` (`LevelSequenceActor.DefaultInstanceData` _outactor)))
  (set `DefaultLevelSequenceInstanceData.TransformOrigin` (`KismetMathLibrary.MakeTransform` (`self.K2_GetActorLocation` (`self.Unit`))) _asdefault_level_sequence_instance_data)
  (`LevelSequenceActor.SetBindingByTag` _outactor "Unit" (`|MakeArray` (`self.Unit`) :!type "Actor Object Reference") false)
  (`MovieSceneSequencePlayer.Play` _returnvalue))

(fn `UserConstructionScript`)