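; BP_Effect_Slash is a melee slash ability effect that plays a greatsword attack montage on the casting unit.
; On each montage notify it fans line traces from the floor under the unit, starting at minus half the ability angle and reaching out to placement range.
; Every trace applies calculated damage to its hit actor without de-duplication.
; When the montage completes, the effect signals completion and destroys itself.
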(event `self.ReceiveBeginPlay`
  (bind _unit (`self.Unit`))
  (bind (_floorresult_bblockinghit _floorresult_bwalkablefloor _floorresult_blinetrace _floorresult_floordist _floorresult_linedist _floorresult_hitresult) (break `FindFloorResult` (`CharacterMovementComponent.K2_FindFloor` (`Character.CharacterMovement` _unit) (`self.K2_GetActorLocation` _unit))))
  (bind (_bblockinghit _binitialoverlap _time _distance _location) (`GameplayStatics.BreakHitResult` _floorresult_hitresult))
  (`parent.ReceiveBeginPlay`)
  (`|PlayMontage` (`Character.Mesh` (`self.Unit`)) "/Game/Game/Blueprints/Units/Animations/Frank_RPG_GreatSword_Attack03_Montage.Frank_RPG_GreatSword_Attack03_Montage"
    (:`OnCompleted`
      (`self.OnEffectCompleted` self)
      (`self.K2_DestroyActor`))
    (:`OnNotifyBegin`
      (for _index (range (+ (`KismetMathLibrary.FTrunc` (* (/ (`/Game/Game/Blueprints/Abilities/Data/PDA_Action.Angle` (`self.AbilityData`)) 5.0) 2.0)) 1))
        (bind _outhit (`KismetSystemLibrary.LineTraceSingle` _location (+ _location (* (`KismetMathLibrary.GreaterGreater_VectorRotator` (`KismetMathLibrary.GetForwardVector` (`self.K2_GetActorRotation` _unit)) (`KismetMathLibrary.MakeRotator` 0.0 0.0 (- (* _index 2.0) (/ (`/Game/Game/Blueprints/Abilities/Data/PDA_Action.Angle` (`self.AbilityData`)) 2.0)))) (`/Game/Game/Blueprints/Abilities/Data/PDA_Action.PlacementRange` (`self.AbilityData`)))) "TraceTypeQuery3" false (`|MakeArray` (`self.Unit`) :!type "Actor Object Reference") "ForOneFrame"))
        (bind _returnvalue (`/Game/Game/Blueprints/Abilities/Data/PDA_Action.CalculateDamage` (`self.AbilityData`) 1.0))
        (`GameplayStatics.ApplyDamage` (`.HitActor` (`GameplayStatics.BreakHitResult` _outhit)) _returnvalue null self)))))

(fn `UserConstructionScript`
  (`parent.UserConstructionScript`))