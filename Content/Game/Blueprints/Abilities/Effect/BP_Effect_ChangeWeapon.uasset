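; BP_Effect_ChangeWeapon is an ability effect that swaps its owner's weapon to the Crossbow for as long as the effect exists.
; On BeginPlay it caches the current weapon from the owner's AC_Loadout component, then equips the Crossbow through that component.
; When destroyed, it re-equips the cached weapon, so the effect's lifetime sets the duration of the swap.
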(event `self.ReceiveBeginPlay`
  (bind _returnvalue (`self.GetComponentByClass` (`self.GetOwner`) "/Game/Game/System/Components/AC_Loadout.AC_Loadout_C"))
  (`parent.ReceiveBeginPlay`)
  (set `self.Equipped Weapon` (`/Game/Game/System/Components/AC_Loadout.GetWeapon` _returnvalue))
  (`/Game/Game/System/Components/AC_Loadout.EquipWeapon` _returnvalue "/Game/Game/Blueprints/Loadout/Weapons/Data/Range/Crossbow.Crossbow" "None"))

(event `self.ReceiveDestroyed`
  (`/Game/Game/System/Components/AC_Loadout.EquipWeapon` (`self.GetComponentByClass` (`self.GetOwner`) "/Game/Game/System/Components/AC_Loadout.AC_Loadout_C") (`self.Equipped Weapon`) "None"))

(fn `UserConstructionScript`
  (`parent.UserConstructionScript`))