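; BP_Effect_Heal is an ability effect actor named for healing, though its own graph only issues a unit move.
; On BeginPlay, after the parent logic, the authority orders Unit to a random reachable point within a tiny radius of the effect, then binds to its move-ended event.
; When the move ends, regardless of success, it signals effect completion and destroys itself.
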(event `self.ReceiveBeginPlay`
  (bind _unit (`self.Unit`))
  (`parent.ReceiveBeginPlay`)
  (`/Engine/EditorBlueprintResources/ActorMacros.Switch Has Authority`
    (:`Authority`
      (`/Game/Game/Blueprints/Units/BP_Unit.Command_Move` _unit (`NavigationSystemV1.K2_GetRandomReachablePointInRadius` (`self.K2_GetActorLocation`) 10.0 null null))
      (add `/Game/Game/Blueprints/Units/BP_Unit.OnMoveEnded` _unit (delegate `OnMoveEnded`)))))

(event `OnMoveEnded`
  (params (Success :type Boolean))
  (`self.OnEffectCompleted` self)
  (`self.K2_DestroyActor`))

(fn `UserConstructionScript`
  (`parent.UserConstructionScript`))