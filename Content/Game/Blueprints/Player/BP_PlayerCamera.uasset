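; Player camera actor that becomes the first player's view target on BeginPlay and enables that controller's input on itself.
; Enhanced Input actions pan it along its local X/Y axes, scaled by CameraSpeed, and yaw it in world space by 45-degree multiples of the input.
; FocusCamera snaps it to a valid target actor's location and sets the spring arm length to the given distance.
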(event `self.ReceiveBeginPlay`
  (bind _returnvalue (`GameplayStatics.GetPlayerController` 0))
  (`PlayerController.SetViewTargetWithBlend` _returnvalue self 0.0 "VTBlend_Linear" 0.0 false)
  (`self.EnableInput` _returnvalue))

(event `EnhancedInput|/Game/Game/System/Inputs/IA_PanCamera`
  (params (ActionValue :type "Vector2D Structure") (ElapsedSeconds :type "Float (double-precision)") (TriggeredSeconds :type "Float (double-precision)") (InputAction :type "InputAction Object Reference" :default "/Game/Game/System/Inputs/IA_PanCamera.IA_PanCamera"))
  (bind (_returnvalue_x _returnvalue_y) (`KismetMathLibrary.BreakVector2D` (* ActionValue (`self.CameraSpeed`))))
  (:`Triggered`
    (`self.K2_AddActorLocalOffset` (`KismetMathLibrary.MakeVector` _returnvalue_x _returnvalue_y))))

(event `EnhancedInput|/Game/Game/System/Inputs/IA_RotateCamera`
  (params (ActionValue :type "Float (double-precision)") (ElapsedSeconds :type "Float (double-precision)") (TriggeredSeconds :type "Float (double-precision)") (InputAction :type "InputAction Object Reference" :default "/Game/Game/System/Inputs/IA_RotateCamera.IA_RotateCamera"))
  (:`Triggered`
    (`self.K2_AddActorWorldRotation` (`KismetMathLibrary.MakeRotator` 0.0 0.0 (* ActionValue 45.0)))))

(event `FocusCamera`
  (params (Actor :type "Actor Object Reference") (Distance :type "Float (double-precision)"))
  (`/Engine/EditorBlueprintResources/StandardMacros.IsValid` Actor
    (:`Is Valid`
      (`self.K2_SetActorLocation` (`self.K2_GetActorLocation` Actor))
      (set `SpringArmComponent.TargetArmLength` Distance (`self.SpringArm`)))))

(fn `UserConstructionScript`)