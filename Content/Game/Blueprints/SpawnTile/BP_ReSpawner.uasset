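; BP_ReSpawner is a respawn tile for the turn-based game that shows its cube only when it is a valid respawn spot.
; It listens to the game state's phase changes and shows the cube during one specific phase if the local player's unit is dead.
; A range check filters player units by team and hides the cube when the nearest opposing unit is within a fixed distance.
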(event `self.ReceiveBeginPlay`
  ;[1 0 0] use parent begin play and then just use event on phase change!?
  (bind _asgs_turn_based (cast `/Game/Game/System/Gameplay/GS_TurnBased` (`GameplayStatics.GetGameState`)))
  (add `/Game/Game/System/Gameplay/GS_TurnBased.OnPhaseChanged` _asgs_turn_based (delegate `OnPhaseChanged`)))

(event `OnPhaseChanged`
  (params (Phase :type "/Game/Game/System/Enums/EPhase Enum" :default "NewEnumerator5"))
  (bind _cube (`self.Cube`))
  ;[1 0 0] use parent begin play and then just use event on phase change!?
  (if (`|EnumEquality` Phase "NewEnumerator1")
    (bind _aspc_turn_based (cast `/Game/Game/System/Gameplay/PC_TurnBased` (`GameplayStatics.GetPlayerController` 0)))
    (if (`/Game/Game/System/Gameplay/PC_TurnBased.IsUnitDead` _aspc_turn_based)
      (if (`self.IsInRangeOfEnemy`)
        (`SceneComponent.SetVisibility` _cube false false)
        (else
          (`SceneComponent.SetVisibility` _cube true false)))
      (else
        (`SceneComponent.SetVisibility` _cube false false)))
    (else
      (`SceneComponent.SetVisibility` _cube false false))))

(event `self.OnPhaseChange`
  (params (Phase :type "/Game/Game/System/Enums/EPhase Enum" :default "NewEnumerator5"))
  ;[1 0 0] use parent begin play and then just use event on phase change!?
)

(fn `Find Actor Within Distance`
  (params (ActorsToCheck :type "Array of Actor Object Reference (by ref)") (Distance :type "Float (double-precision)"))
  (returns (`Success?` :type Boolean))
  (return (< (`GameplayStatics.FindNearestActor` (`self.K2_GetActorLocation`) ActorsToCheck) Distance)))

(fn `IsInRangeOfEnemy`
  (returns (ReturnValue :type Boolean))
  (locals (LocMyTeam :type "/Game/Game/System/Enums/ETeam Enum" :default "NewEnumerator0") (Local_AllUnits :type "Array of /Game/Game/Blueprints/Units/Player/BP_Unit_Player Object Reference") (Local__WorkingList :type "Array of /Game/Game/Blueprints/Units/Player/BP_Unit_Player Object Reference"))
  (bind _asps_turn_based (cast `/Game/Game/System/Gameplay/PS_TurnBased` (`Controller.PlayerState` (`GameplayStatics.GetPlayerController` 0))))
  (set `local.LocMyTeam` (`/Game/Game/System/Gameplay/PS_TurnBased.Team` _asps_turn_based))
  (bind _outactors (`GameplayStatics.GetAllActorsOfClass` "/Game/Game/Blueprints/Units/Player/BP_Unit_Player.BP_Unit_Player_C"))
  (bind _output_get (set `local.Local_AllUnits` _outactors))
  (set `local.Local__WorkingList` _output_get)
  (for (_array_element _array_index) _output_get
    ;[1 1 1] Remove Array Indix for non Matching Team
    (if (`|EnumEquality` (`/Game/Game/System/Components/AC_Attributes.Team` (`/Game/Game/Blueprints/Units/BP_Unit.AC_Attributes` _array_element)) (`local.LocMyTeam`))
      (`KismetArrayLibrary.Array_Remove` (`local.Local__WorkingList`) _array_index)))
  (bind _success_ (`self.Find Actor Within Distance` (`local.Local__WorkingList`) 500.0))
  (return _success_))

(fn `UserConstructionScript`
  (`parent.UserConstructionScript`))