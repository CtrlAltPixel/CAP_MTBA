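; BP_Magic is a base Blueprint for magic in the loadout system, with ApplyMagic left empty for child classes to override.
; AttemptApplication calls ApplyMagic only when CheckTagCondition passes.
; That check reads active tags from an AC_GameplayTags component, requiring all RequiredTags and none of the PreventingTags, with non-exact matching.
; BeginPlay only validates MagicData and takes no further action.
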(event `self.ReceiveBeginPlay`
  (`self.MagicData`
    (:`then`)
    (:`else`)))

(event `AttemptApplication`
  (bind _bsuccess_ (`self.CheckTagCondition`))
  (if _bsuccess_
    (`self.ApplyMagic`)))

(event `ApplyMagic`
  ;[1 1 1] Overwrite in children
)

(fn `CheckTagCondition`
  (returns (`bSuccess?` :type Boolean))
  (bind _returnvalue (`self.GetComponentByClass` "/Game/Game/System/Components/AC_GameplayTags.AC_GameplayTags_C"))
  (`/Engine/EditorBlueprintResources/StandardMacros.IsValid` _returnvalue
    (:`Is Valid`
      (bind _tagcontainer (`/Game/Game/System/Components/AC_GameplayTags.GetActiveTagContainer` _returnvalue))
      (return (and (`BlueprintGameplayTagLibrary.HasAllTags` _tagcontainer (`self.RequiredTags`)) (not (`BlueprintGameplayTagLibrary.HasAnyTags` _tagcontainer (`self.PreventingTags`))))))))

(fn `UserConstructionScript`)