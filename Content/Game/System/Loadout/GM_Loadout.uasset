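; Game mode for the loadout phase between the lobby and the arena match.
; Tracks logged-in players and announces each join, including controllers swapped in from the lobby, which inherit the old controller's team message.
; A one-shot timer starts at BeginPlay with the maximum loadout time, and its end event server-travels to LVL_Arena01.
; Copying settings and player data to the loadout controller is left unconnected.
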(event `self.K2_PostLogin`
  (params (NewPlayer :type "PlayerController Object Reference"))
  (`KismetArrayLibrary.Array_AddUnique` (`self.ConnectedPlayers`) NewPlayer)
  (`self.OnPlayerJoined` NewPlayer))

(event `self.K2_OnSwapPlayerControllers`
  (params (OldPC :type "PlayerController Object Reference") (NewPC :type "PlayerController Object Reference"))
  ;[1 0 0] are we still setting this as previously as to read from a save game data?
  (bind _aspc_lobby (cast `/Game/Game/System/Lobby/PC_Lobby` OldPC))
  (bind _team (message `/Game/Game/System/Interfaces/BPI_Team.GetTeam` OldPC))
  (message `/Game/Game/System/Interfaces/BPI_Team.SetTeam` NewPC _team)
  (`self.OnPlayerJoined` NewPC))

(event `self.ReceiveBeginPlay`
  (bind _returnvalue (`KismetSystemLibrary.K2_SetTimerDelegate` (`|CreateDelegate` :!event `EndLoadoutTimer`) (`self.MaxLoadoutTime`)))
  (set `self.LoadoutTimer` _returnvalue))

(event `EndLoadoutTimer`
  (`KismetSystemLibrary.ExecuteConsoleCommand` "servertravel Game/Game/Maps/LVL_Arena01" (`GameplayStatics.GetPlayerController` 0)))

(fn `UserConstructionScript`)