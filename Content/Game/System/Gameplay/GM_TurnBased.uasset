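; GM_TurnBased is the game mode for turn-based play, passing player joins and unit deaths to the game state.
; On begin play it caches GS_TurnBased and binds an OnUnitDied handler.
; Logins notify the cached game state of the new player controller.
; Unit deaths update victim and killer and announce the kill through the game state, re-fetching it if the cached reference is invalid.
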(event `self.ReceiveBeginPlay`
  ;[1 0 0] Add unit death and team score
  (bind _asgs_turn_based (cast `/Game/Game/System/Gameplay/GS_TurnBased` (`GameplayStatics.GetGameState`)))
  (set `self.As GS Turn Based` _asgs_turn_based)
  (add `self.OnUnitDied` (`|CreateDelegate` :!event `UnitDied`)))

(event `self.K2_PostLogin`
  (params (NewPlayer :type "PlayerController Object Reference"))
  (bind _aspc_turn_based (cast `/Game/Game/System/Gameplay/PC_TurnBased` NewPlayer))
  (bind _as_gs_turn_based (`self.As GS Turn Based`)
    (:`then`
      (`/Game/Game/System/Gameplay/GS_TurnBased.NewPlayerConnected` _as_gs_turn_based _aspc_turn_based))
    (:`else`)))

(event `UnitDied` :!signature `self.OnUnitDied`
  (params (KilledUnit :type "/Game/Game/Blueprints/Units/BP_Unit Object Reference") (DamageCauser :type "Actor Object Reference"))
  (bind _as_gs_turn_based (`self.As GS Turn Based`))
  ;[1 0 0] Should this include input for controller/playerstate maybe look into updating the on unit died call? should the cast to game state exist here?
  (bind _as_gs_turn_based_2 (`self.As GS Turn Based`)
    (:`then`
      _)
    (:`else`
      (bind _asgs_turn_based (cast `/Game/Game/System/Gameplay/GS_TurnBased` (`GameplayStatics.GetGameState`)))
      (bind _output_get (set `self.As GS Turn Based` _asgs_turn_based))))
  (`/Game/Game/System/Gameplay/GS_TurnBased.UpdateUnitVictim` _as_gs_turn_based_2 KilledUnit)
  (`/Game/Game/System/Gameplay/GS_TurnBased.UpdateUnitVictim` _output_get KilledUnit)
  (`/Game/Game/System/Gameplay/GS_TurnBased.UpdateUnitKiller` _as_gs_turn_based null)
  (`/Game/Game/System/Gameplay/GS_TurnBased.AnnounceKill` _as_gs_turn_based KilledUnit DamageCauser))

(event `self.K2_OnLogout`
  (params (ExitingController :type "Controller Object Reference")))

(fn `UserConstructionScript`)