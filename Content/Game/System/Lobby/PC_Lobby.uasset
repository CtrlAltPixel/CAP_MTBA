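; Lobby player controller that shows the custom lobby HUD for the local player and handles team selection.
; On BeginPlay it creates the widget, switches to UI-only input and shows the cursor.
; SetTeam forwards to a server event that asks GS_Lobby to assign the team, storing it on success or printing a client-side error on failure.
; The Team RepNotify passes the value to a player state via an interface-style message.
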(event `self.ReceiveBeginPlay`
  ;[1 0 0] Does this need to be set to Lobby HUD?
  (if (`self.IsLocalController`)
    (bind _returnvalue (`|CreateWidget` "/Game/Game/UI/Lobby/Custom/WB_CustomLobbyHUD.WB_CustomLobbyHUD_C"))
    (bind _output_get (set `self.AsLobbyHUD` _returnvalue))
    (`UserWidget.AddToViewport` _output_get 0)
    (`WidgetBlueprintLibrary.SetInputMode_UIOnlyEx` self _output_get)
    (set `self.bShowMouseCursor` true)))

(event `/Game/Game/System/Interfaces/BPI_Team.SetTeam`
  (params (Team :type "/Game/Game/System/Enums/ETeam Enum" :default "NewEnumerator0"))
  (`self.SERVER_AssignControllerToTeam` Team))

(event `SERVER_AssignControllerToTeam`
  (params (`Team To Assign` :type "/Game/Game/System/Enums/ETeam Enum" :default "NewEnumerator0"))
  (bind _asgs_lobby (cast `/Game/Game/System/Lobby/GS_Lobby` (`GameplayStatics.GetGameState`)))
  (bind _success (`/Game/Game/System/Lobby/GS_Lobby.Assign Player To Team` _asgs_lobby `Team To Assign` self))
  (if _success
    (set `self.Team` `Team To Assign`)
    (else
      (`self.CLIENT_DIsplayError` "Failed to join Team"))))

(event `CLIENT_DIsplayError`
  (params (Error :type String))
  (`KismetSystemLibrary.PrintString` Error))

(fn `GetTeam`
  (returns (Team :type "/Game/Game/System/Enums/ETeam Enum"))
  (return (`self.Team`)))

(fn `OnRep_Team`
  (message `/Game/Game/System/Interfaces/BPI_Team.SetTeam` (`GameplayStatics.GetPlayerState` 0) (`self.Team`)))

(fn `UserConstructionScript`)