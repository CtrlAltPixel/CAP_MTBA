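; Player controller for a networked turn-based game, handling click interaction and the player's unit.
; Clicks trace under the cursor locally, then a server event messages the hit actor to interact.
; Game state phase changes drive Preparation: the server spawns the loadout unit at the assigned spawner, and local players focus the camera on it.
; RepNotifies bind server phase handling, move the view to the unit and set the host's team; movement abilities spawn on demand.
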(event `self.ReceiveBeginPlay`
  ;[1 1 1] BeginPlay
  (if (`self.IsLocalPlayerController`)
    (`EnhancedInputSubsystemInterface.AddMappingContext` (pcsubsystem `EnhancedInputLocalPlayerSubsystem` self) "/Game/Game/System/Inputs/IC_TurnBased.IC_TurnBased" 0 (struct))
    (bind _asgs_turn_based (cast `/Game/Game/System/GS_TurnBased` (`GameplayStatics.GetGameState`)))
    (add `/Game/Game/System/GS_TurnBased.OnPhaseChanged` _asgs_turn_based (`|CreateDelegate` :!event `OnPhaseChange`))))

(event `EnhancedInput|/Game/Game/System/Inputs/IA_SingleClick`
  (params (ActionValue :type Boolean) (ElapsedSeconds :type "Float (double-precision)") (TriggeredSeconds :type "Float (double-precision)") (InputAction :type "InputAction Object Reference" :default "/Game/Game/System/Inputs/IA_SingleClick.IA_SingleClick"))
  ;[1 1 1] Click Event
  (:`Triggered`
    (bind _output_get (set `self.InteractActor` (`.HitActor` (`GameplayStatics.BreakHitResult` (`self.GetHitResultUnderCursorByChannel` "TraceTypeQuery1")))))
    (`self.SERVER_Click` _output_get)))

(event `SERVER_Click`
  (params (Actor :type "Actor Object Reference"))
  ;[1 1 1] Click Event
  (message `/Game/Game/System/BPI_Interaction.InteractWith` Actor self))

(event `OnPhaseChange`
  (params (Phase :type "/Game/Game/System/Enums/EPhase Enum" :default "NewEnumerator5"))
  ;[1 1 1] On Phase Change
  (switch `/Game/Game/System/Enums/EPhase` Phase
    (:`NewEnumerator0`
      (bind _returnvalue (`GameplayStatics.GetActorOfClass` "/Game/Game/Blueprints/Player/BP_PlayerCamera.BP_PlayerCamera_C"))
      (`/Game/Game/Blueprints/Player/BP_PlayerCamera.FocusCamera` _returnvalue (`self.CurrentUnit`) 500.0))))

(event `SpawnMovementAbility`
  (params (AbilityData :type "/Game/Game/Blueprints/Abilities/Data/DA_Ability Object Reference"))
  (bind _currentunit (`self.CurrentUnit`))
  ;[1 1 1] Comment
  (`self.CurrentUnit`
    (:`then`
      (`self.MovementAbility`
        (:`then`
          (`self.K2_DestroyActor` (`self.MovementAbility`)))
        (:`else`
          _))
      (bind _returnvalue (`|SpawnActorFromClass` (`/Game/Game/Blueprints/Abilities/Data/DA_Ability.AbilityClass` AbilityData) (`self.GetTransform` _currentunit) "AlwaysSpawn" "MultiplyWithRoot" self _currentunit null))
      (set `self.MovementAbility` _returnvalue))
    (:`else`)))

(fn `OnRep_CurrentUnit`
  (`self.K2_SetActorLocation` (`self.GetViewTarget`) (`self.K2_GetActorLocation` (`self.CurrentUnit`)) false false)
  (`/Engine/EditorBlueprintResources/ActorMacros.Switch Has Authority`
    (:`Authority`
      (if (`self.IsLocalController`)
        (set `/Game/Game/Blueprints/Components/AC_Stats.Team` "NewEnumerator2" (`/Game/Game/Blueprints/Units/BP_Unit.AC_Stats` (`self.CurrentUnit`)))))))

(fn `OnRep_Spawner`
  (`/Engine/EditorBlueprintResources/ActorMacros.Switch Has Authority`
    (:`Authority`
      (bind _asgs_turn_based (cast `/Game/Game/System/GS_TurnBased` (`GameplayStatics.GetGameState`)))
      (`/Game/Game/System/GS_TurnBased.AreAllPlayersReady` _asgs_turn_based)
      (add `/Game/Game/System/GS_TurnBased.OnPhaseChanged` _asgs_turn_based (`|CreateDelegate` :!event `Phase Changed`)))))

(fn `Phase Changed`
  (params (Phase :type "/Game/Game/System/Enums/EPhase Enum" :default "NewEnumerator5"))
  (switch `/Game/Game/System/Enums/EPhase` Phase
    (:`NewEnumerator0`
      (`self.UnitSpawn`))))

(fn `UnitSpawn`
  (`self.CurrentUnit`
    (:`then`)
    (:`else`
      (bind _returnvalue (`|SpawnActorFromClass` (`.UnitClass_2_17AED7144010AC87D7CB23A95E607AEE` (break `/Game/Game/System/Structs/FLoadout` (`self.Loadout`))) (`self.GetTransform` (`self.Spawner`)) "AdjustIfPossibleButAlwaysSpawn" "MultiplyWithRoot" (`self.GetOwner`) null))
      (bind _output_get (set `self.CurrentUnit` _returnvalue))
      (`self.OnUnitCreated` _output_get)
      (set `/Game/Game/Blueprints/Units/BP_Unit.UnitName` (`PlayerState.GetPlayerName` (`self.PlayerState`)) _output_get))))

(fn `UserConstructionScript`)