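; Actor component that tracks a unit's gameplay tags for controller, state and team, with reference-counted stacks per tag.
; Add and remove update a name-keyed count map and the active container, dropping a tag at zero and printing debug counts.
; A switch macro routes NotifyTagChange to per-tag dispatchers carrying tag and origin.
; AddTagListener binds only AI, Dead and Knockdown, with AI bound to the Attacking dispatcher; add/remove never notify.
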(event `Signature` :!signature `self.OnDeadChange`
  (params (`Gameplay Tag Context` :type "/Game/Game/System/Structs/FGameplayTagContext Structure"))
  ;[1 1 1] Placeholder to allow copying of signature in EventDispatchers
)

(fn `AddGameplayTag`
  (params (TagToAdd :type "GameplayTag Structure") (Origin :type "/Game/Game/System/Structs/FOrigin Structure"))
  (`self.AddTagToStack` TagToAdd 1)
  (`BlueprintGameplayTagLibrary.AddGameplayTag` (`self.ActiveTags`) TagToAdd)
  (`self.DEBUG Print Stack Count` TagToAdd "AC_GameplayTags")
  (return))

(fn `AddTagListener`
  (params (TagToListenFor :type "GameplayTag Structure") (Event :type "Delegate (by ref)"))
  (`self.DetermineTagChange` TagToListenFor
    (:`AIChange`
      (add `self.OnAttackingChange` (`local.Event`)))
    (:`DeadChange`
      (add `self.OnDeadChange` (`local.Event`)))
    (:`KnockdownChange`
      (add `self.OnKnockdownChange` (`local.Event`)))))

(fn `AddTagToStack`
  (params (TagToAdd :type "GameplayTag Structure") (QuantityToAdd :type Integer))
  (bind _returnvalue (`BlueprintGameplayTagLibrary.GetTagName` TagToAdd))
  (bind _tagstack (`self.TagStack`))
  (`BlueprintMapLibrary.Map_Add` _tagstack _returnvalue (+ (`BlueprintMapLibrary.Map_Find` _tagstack _returnvalue) QuantityToAdd))
  (return))

(fn `CreateContext`
  (params (ContextTag :type "GameplayTag Structure") (Origin :type "/Game/Game/System/Structs/FOrigin Structure"))
  (returns (GameplayContext :type "/Game/Game/System/Structs/FGameplayTagContext Structure"))
  (return (make `/Game/Game/System/Structs/FGameplayTagContext` ContextTag (struct) Origin)))

(fn `DEBUG Print Stack Count`
  (params (TagToPrint :type "GameplayTag Structure") (DebugLocation :type String))
  (bind _returnvalue (`BlueprintGameplayTagLibrary.GetTagName` TagToPrint))
  (`KismetSystemLibrary.PrintString` (`KismetStringLibrary.Concat_StrStr` DebugLocation "Stack amount of:" (`KismetStringLibrary.Conv_NameToString` _returnvalue) (`KismetStringLibrary.Conv_IntToString` (`BlueprintMapLibrary.Map_Find` (`self.TagStack`) _returnvalue))) true true (struct :`G` 0.66 :`B` 1.0 :`A` 1.0) 5.0)
  (return))

(fn `GetActiveTagContainer`
  (returns (TagContainer :type "GameplayTagContainer Structure"))
  (return (`self.ActiveTags`)))

(fn `NotifyTagChange`
  (params (TagToListenFor :type "GameplayTag Structure") (Origin :type "/Game/Game/System/Structs/FOrigin Structure"))
  (locals (Local_GamplayTagContext :type "/Game/Game/System/Structs/FGameplayTagContext Structure"))
  (bind _gameplaycontext (`self.CreateContext` TagToListenFor Origin))
  (set `local.Local_GamplayTagContext` _gameplaycontext)
  (`self.DetermineTagChange` TagToListenFor
    (:`AIChange`
      (`self.OnAIChange` (`local.Local_GamplayTagContext`))
      (return))
    (:`PlayerChange`
      (`self.OnPlayerChange` (`local.Local_GamplayTagContext`))
      (return))
    (:`AttackingChange`
      (`self.OnAttackingChange` (`local.Local_GamplayTagContext`))
      (return))
    (:`DeadChange`
      (`self.OnDeadChange` (`local.Local_GamplayTagContext`))
      (return))
    (:`KnockdownChange`
      (`self.OnKnockdownChange` (`local.Local_GamplayTagContext`))
      (return))
    (:`EnemyTeamChange`
      (`self.OnEnemyChange` (`local.Local_GamplayTagContext`))
      (return))
    (:`FriendlyTeamChange`
      (`self.OnFriendlyChange` (`local.Local_GamplayTagContext`))
      (return))))

(fn `RemoveGameplayTag`
  (params (TagToRemove :type "GameplayTag Structure") (Origin :type "/Game/Game/System/Structs/FOrigin Structure"))
  (bind _bisempty_ (`self.RemoveTagFromStack` TagToRemove 1))
  (if _bisempty_
    (`BlueprintGameplayTagLibrary.RemoveGameplayTag` (`self.ActiveTags`) TagToRemove))
  (`self.DEBUG Print Stack Count` TagToRemove "AC_GameplayTags")
  (return))

(fn `RemoveTagFromStack`
  (params (TagToRemove :type "GameplayTag Structure") (QuantityToRemove :type Integer))
  (returns (`bIsEmpty?` :type Boolean))
  (locals (Local_StackCount :type Integer :default 0))
  (bind _returnvalue (`BlueprintGameplayTagLibrary.GetTagName` TagToRemove))
  (bind _tagstack (`self.TagStack`))
  (bind _output_get (set `local.Local_StackCount` (`KismetMathLibrary.Clamp` (- (`BlueprintMapLibrary.Map_Find` _tagstack _returnvalue) QuantityToRemove) 0 999)))
  (`BlueprintMapLibrary.Map_Add` _tagstack _returnvalue _output_get)
  (if (<= (`local.Local_StackCount`) 0)
    (`BlueprintMapLibrary.Map_Remove` _tagstack _returnvalue)
    (return true)
    (else
      (return false))))