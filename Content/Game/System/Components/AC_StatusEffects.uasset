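; Actor component that keeps the list of status effects active on its owner.
; Adding an effect stores it, broadcasts OnAddStatusEffect, then asks the effect to attempt its own application.
; Removing an effect broadcasts OnRemoveStatusEffect only if it was in the list, and makes no call on the effect itself.
; AddStatusEffectListener is an empty stub, and the event graph holds no live logic.
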(event `StatusEffectSignature` :!signature `self.OnAddStatusEffect`
  (params (StatusEffectAdded :type "/Game/Game/Blueprints/StatusEffects/BP_Statuseffects Object Reference"))
  ;[1 1 1] Used To  Create Signature for EventDispatcher
)

(fn `Add Status Effect`
  (params (StatusEffectToAdd :type "/Game/Game/Blueprints/StatusEffects/BP_Statuseffects Object Reference (by ref)"))
  (`KismetArrayLibrary.Array_Add` (`self.ActiveStatusEffects`) StatusEffectToAdd)
  (`self.OnAddStatusEffect` StatusEffectToAdd)
  (`/Game/Game/Blueprints/StatusEffects/BP_Statuseffects.AttemptApplication` StatusEffectToAdd))

(fn `AddStatusEffectListener`)

(fn `GetStatusEffects`
  (returns (ActiveStatusEffects :type "Array of /Game/Game/Blueprints/StatusEffects/BP_Statuseffects Object Reference"))
  (return (`self.ActiveStatusEffects`)))

(fn `RemoveStatusEffect`
  (params (StatusEffectToRemove :type "/Game/Game/Blueprints/StatusEffects/BP_Statuseffects Object Reference (by ref)"))
  (bind _returnvalue (`KismetArrayLibrary.Array_RemoveItem` (`self.ActiveStatusEffects`) StatusEffectToRemove))
  (if _returnvalue
    (`self.OnRemoveStatusEffect` StatusEffectToRemove)
    (return)))