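; AC_Abilities is an actor component that holds the list of current actions (abilities) for its owning Pawn, which it caches on BeginPlay.
; Initialise, add and remove functions edit the list, with add and remove broadcasting the updated array through a change dispatcher.
; UseAbility and ActivateAction are empty stubs, and the available-action change binding is never executed.
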(event `self.ReceiveBeginPlay`
  ;[1 0 0] Should I do this/ Is it needed?
  (bind _aspawn (cast `Pawn` (`self.GetOwner`)))
  (set `self.As Owning Pawn Reference` _aspawn))

(event `ActivateAction`)

(event `AvailableAbilitiesChangeSignature` :!signature `self.OnAvailableActionChange`
  (params (NewParam :type "Array of /Game/Game/Blueprints/Abilities/Data/PDA_Action Object Reference (by ref)"))
  ;[1 1 1] Comment
)

(fn `Add Action`
  (params (ActionToAdd :type "/Game/Game/Blueprints/Abilities/Data/PDA_Action Object Reference"))
  (`KismetArrayLibrary.Array_Add` (`self.CurrentActions`) ActionToAdd)
  (`self.OnCurrentActionsChange` (`self.CurrentActions`))
  (return))

(fn `InitialiseActions`
  (params (KnownActions :type "Array of /Game/Game/Blueprints/Abilities/Data/PDA_Action Object Reference"))
  (for _array_element KnownActions
    (`self.Add Action` _array_element))
  (return))

(fn `Remove Action`
  (params (AbilityToRemove :type "/Game/Game/Blueprints/Abilities/Data/PDA_Action Object Reference"))
  (for _array_element (`self.CurrentActions`)
    (if (== _array_element AbilityToRemove)
      (`KismetArrayLibrary.Array_RemoveItem` (`self.CurrentActions`) _array_element)))
  (`self.OnCurrentActionsChange` (`self.CurrentActions`))
  (return))

(fn `UseAbility`
  (params (ActionIndex :type Integer))
  (return))