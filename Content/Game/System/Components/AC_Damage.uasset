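; Damage component that deals damage to other actors and turns damage taken by its owner into health changes.
; On BeginPlay it binds to the owner's OnTakeAnyDamage, provided the owner is a Pawn with AC_Attributes.
; Incoming damage is calculated by the DamageType's UpdateDamageMessage, then applied to Attribute.Health.Current through AC_Attributes.
; AttemptDamage hits each actor only once, tracked in a DamagedActors array that is never cleared here.
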(event `self.ReceiveBeginPlay`
  (bind _returnvalue (`self.GetOwner`))
  (`/Engine/EditorBlueprintResources/StandardMacros.IsValid` (`Actor.GetComponentByClass` _returnvalue "/Game/Game/System/Components/AC_Attributes.AC_Attributes_C")
    (:`Is Valid`
      (bind _aspawn (cast `Pawn` _returnvalue))
      (set `self.As Pawn Reference` _aspawn)
      (add `Actor.OnTakeAnyDamage` _returnvalue (`|CreateDelegate` :!event `OnOwnerTakeDamage`)))))

(event `AttemptDamage`
  (params (Actor :type "Actor Object Reference"))
  ;[1 0 0] Might be better replaced with BP_Unit DamageCooldown event oitherwise need to clear array somewhere
  (if (not (`KismetArrayLibrary.Array_Contains` (`self.DamagedActors`) Actor))
    (`KismetArrayLibrary.Array_Add` (`self.DamagedActors`) Actor)
    (`GameplayStatics.ApplyDamage` Actor)))

(event `OnOwnerTakeDamage`
  (params (DamagedActor :type "Actor Object Reference") (Damage :type "Float (single-precision)") (DamageType :type "DamageType Object Reference") (InstigatedBy :type "Controller Object Reference") (DamageCauser :type "Actor Object Reference"))
  (bind _returnvalue (`Actor.GetComponentByClass` DamagedActor "/Game/Game/System/Components/AC_Attributes.AC_Attributes_C"))
  (`/Engine/EditorBlueprintResources/StandardMacros.IsValid` _returnvalue
    (:`Is Valid`
      (bind _output_get (set `self.Damage Type` DamageType))
      ;[1 0 0] check dmg is negative and change target input to a pawn ref not unit?
      (bind (_calculateddamage _damagetype) (message `/Game/Game/Blueprints/DamageTypes/Interface/BPI_DamageTypes.UpdateDamage` _output_get Damage null DamageCauser))
      (`/Game/Game/System/Components/AC_Attributes.ChangeAttribute` _returnvalue (struct :`TagName` "Attribute.Health.Current") _calculateddamage "NewEnumerator6" (make `/Game/Game/System/Structs/FOrigin` null)))))