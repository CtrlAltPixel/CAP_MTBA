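; Actor component that holds its owner's loadout: outfit, weapon, glyphs and magic.
; Outfits swap the skeletal mesh on the owner's mesh, fetched through a message call rather than a cast.
; Equipping a weapon removes the old one, spawns a BP_Weapon from weapon data, adds its ability actions and snaps it to a socket.
; Glyph and magic equipping are empty stubs.
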(event `self.ReceiveBeginPlay`)

(fn `EquipGlyphs`
  (params (GlyphsToEquip :type "Map of /Game/Game/System/Enums/EGlyph Enum to Integer")))

(fn `EquipMagic`
  (return))

(fn `EquipOutfit`
  (params (OutfitToEquip :type "SkeletalMesh Object Reference"))
  (bind _skeletalmesh (message `/Game/Game/System/Interfaces/BPI_Loadout.GetMesh` (`self.GetOwner`)))
  (`SkeletalMeshComponent.SetSkeletalMeshAsset` _skeletalmesh OutfitToEquip)
  (set `self.SelectedOutfit` OutfitToEquip)
  (return))

(fn `EquipWeapon`
  (params (WeaponToEquip :type "/Game/Game/Blueprints/Loadout/Weapons/Data/PDA_Weapon Object Reference") (SocketName :type Name))
  (bind _returnvalue (`self.GetOwner`))
  (`/Engine/EditorBlueprintResources/StandardMacros.IsValid` (`Actor.GetComponentByClass` _returnvalue "AC_Loadout_C")
    (:`Is Valid`
      (`self.UnequipWeapon`)
      (bind _returnvalue_2 (`|SpawnActorFromClass` "/Game/Game/Blueprints/Loadout/Weapons/BP_Weapon.BP_Weapon_C" (`KismetMathLibrary.MakeTransform` (0.0 0.0 0.0)) "Undefined" "MultiplyWithRoot" _returnvalue WeaponToEquip null))
      (bind _output_get (set `self.SelectedWeapon` _returnvalue_2))
      (`/Game/Game/Blueprints/Loadout/Weapons/BP_Weapon.AddAbilityActions` _output_get)
      (bind _skeletalmesh (message `/Game/Game/System/Interfaces/BPI_Loadout.GetMesh` (`self.GetOwner`)))
      (`Actor.K2_AttachToComponent` _output_get _skeletalmesh SocketName "SnapToTarget" "SnapToTarget" "SnapToTarget" true)
      (return))))

(fn `GetGlyphs`
  (returns (SelectedGlyphs :type "Map of /Game/Game/System/Enums/EGlyph Enum to Integer"))
  (return (`self.SelectedGlyphs`)))

(fn `GetMagic`
  (returns (SelectedMagic :type "/Game/Game/Blueprints/Loadout/Weapons/BP_Weapon Object Reference"))
  (return (`self.SelectedMagic`)))

(fn `GetOutfit`
  (returns (SelectedMesh :type "SkeletalMesh Object Reference"))
  (return (`self.SelectedOutfit`)))

(fn `GetWeapon`
  (returns (EquippedWeapon :type "/Game/Game/Blueprints/Loadout/Weapons/BP_Weapon Object Reference"))
  (return (`self.SelectedWeapon`)))

(fn `UnequipWeapon`
  (bind _selectedweapon (`self.SelectedWeapon`)
    (:`then`
      (`/Game/Game/Blueprints/Loadout/Weapons/BP_Weapon.RemoveAbilityActions` _selectedweapon)
      (`Actor.K2_DestroyActor` _selectedweapon)
      (set `self.SelectedWeapon` null)
      (return))
    (:`else`)))