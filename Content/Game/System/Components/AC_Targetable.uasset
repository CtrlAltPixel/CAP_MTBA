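; Actor component that makes units damageable, creating their HUD frame and handling incoming damage.
; Damage types implementing BPI_DamageTypes get recalculated damage, which drains Physical or Magic shields before reducing health through AC_Attributes and spawning damage numbers.
; A DoOnce gate re-arms after each hit only while the owner lives, blocking further damage after death.
; Highlight, interaction, target-window and post-damage events are empty stubs, and GetTeam returns a fixed value.
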(event `self.ReceiveBeginPlay`
  ;[1 1 1] Begin Play
  (bind _aspawn (cast `Pawn` (`self.GetOwner`)))
  (set `self.As Pawn Reference` _aspawn)
  (add `Actor.OnTakeAnyDamage` (`self.GetOwner`) (`|CreateDelegate` :!event `PreTakeDamage`))
  ;;[1 0 0] Proimote widget to a variable and need to set the component on unit
  (bind _asbp_unit (cast `/Game/Game/Blueprints/Units/BP_Unit` (`self.GetOwner`)))
  (bind _returnvalue (`|CreateWidget` "/Game/Game/UI/Gameplay/Unit/WB_UnitHUDFrame.WB_UnitHUDFrame_C" null _asbp_unit))
  (`WidgetComponent.SetWidget` (`/Game/Game/Blueprints/Units/BP_Unit.Widget_UnitHUD` _asbp_unit) _returnvalue))

(event `PreTakeDamage`
  (params (DamagedActor :type "Actor Object Reference") (Damage :type "Float (single-precision)") (DamageType :type "DamageType Object Reference") (InstigatedBy :type "Controller Object Reference") (DamageCauser :type "Actor Object Reference"))
  (bind _returnvalue (`self.GetOwner`))
  ;[1 0 0] PreDamage
  (`self.OnPreTakeDamage`)
  (bind _output_get (set `self.Damage Type` DamageType))
  (set `self.Damage Causer` DamageCauser)
  (if (`KismetSystemLibrary.DoesImplementInterface` _output_get "/Game/Game/Blueprints/DamageTypes/Interface/BPI_DamageTypes.BPI_DamageTypes_C")
    (bind _calculateddamage (message `/Game/Game/Blueprints/DamageTypes/Interface/BPI_DamageTypes.UpdateDamage` _returnvalue Damage null _returnvalue))
    (bind _output_get_2 (set `self.LastDamageReceived` _calculateddamage))
    (`self.OnOwnerTakeDamage` null _output_get_2 (`self.Damage Type`) null (`self.Damage Causer`))
    (else
      (set `self.LastDamageReceived` Damage))))

(event `OnOwnerTakeDamage`
  (params (DamagedActor :type "Actor Object Reference") (Damage :type "Float (single-precision)") (DamageType :type "DamageType Object Reference") (InstigatedBy :type "Controller Object Reference") (DamageCauser :type "Actor Object Reference"))
  (bind _returnvalue (`self.GetOwner`))
  (bind _returnvalue_2 (`Actor.GetComponentByClass` DamagedActor "/Game/Game/System/Components/AC_Attributes.AC_Attributes_C"))
  ;[1 0 0] Damage
  (`/Engine/EditorBlueprintResources/StandardMacros.DoOnce` false :!label _label
    (:`Completed`
      (`/Engine/EditorBlueprintResources/StandardMacros.IsValid` _returnvalue_2
        (:`Is Valid`
          (bind _damagehealth (`self.DamageShield` Damage _returnvalue_2))
          (set `self.LastDamageReceived` _damagehealth)
          (bind _attributefound (`/Game/Game/System/Components/AC_Attributes.GetAttributeFromTag` _returnvalue_2 (struct :`TagName` "Attribute.Health.Current")))
          (bind ((`Curent_17_4F1F242B4B6319F1A1C212A3DDC2FAD3` _curent) (`Max_9_CD124E43438FF31CFF85F18B45DE496A` _max)) (break `/Game/Game/System/Structs/FAttributeData` _attributefound))
          (`/Game/Game/System/Components/AC_Attributes.ChangeAttribute` _returnvalue_2 (struct :`TagName` "Attribute.Health.Current") (`KismetMathLibrary.FClamp` (- _curent (`self.LastDamageReceived`)) 0.0 _max) "NewEnumerator6" (make `/Game/Game/System/Structs/FOrigin` _returnvalue (`/Game/Game/Blueprints/Units/BP_Unit.CommandController` (cast `/Game/Game/Blueprints/Units/BP_Unit` _returnvalue :!pure true))))
          (bind _returnvalue_3 (`|CreateWidget` "/Game/Game/UI/Gameplay/WB_DamageNumbers.WB_DamageNumbers_C" null (`self.GetOwner`) (`self.LastDamageReceived`) DamageType))
          (`UserWidget.AddToViewport` _returnvalue_3 0)
          (if (not (`self.IsOwnerDead?`))
            (`self.DamageCooldown`)))))))

(event `DamageCooldown`
  ;[1 0 0] Damage
  (goto _label :!via `Reset`))

(event `PostTakeDamage`
  ;[1 0 0] Post Damage
)

(event `BeginHighlight`
  ;[1 0 0] Highlight and interactions
)

(event `/Game/Game/System/Interfaces/BPI_Interaction.InteractWith`
  (params (PlayerController :type "/Game/Game/System/Gameplay/PC_TurnBased Object Reference"))
  ;[1 0 0] Highlight and interactions
)

(event `EndHighlight`
  ;[1 0 0] Highlight and interactions
)

(event `ShowTargetWindow`
  ;[1 0 0] Highlight and interactions
)

(event `/Game/Game/System/Interfaces/BPI_Interaction.ShowSelectionWindow`
  (params (SelectionFrame :type "UserWidget Object Reference"))
  ;[1 0 0] Highlight and interactions
)

(event `HideTargetWindow`
  ;[1 0 0] Highlight and interactions
)

(fn `DamageShield`
  (params (Damage :type "Float (double-precision)") (AttributesComponent :type "/Game/Game/System/Components/AC_Attributes Object Reference"))
  (returns (DamageHealth :type "Float (double-precision)"))
  (bind _returnvalue (`self.GetOwner`))
  (bind _damage (message `/Game/Game/Blueprints/DamageTypes/Interface/BPI_DamageTypes.GetType` (`self.Damage Type`)))
  (if (or (`|EnumEquality` _damage "NewEnumerator13") (`|EnumEquality` _damage "NewEnumerator15"))
    (bind _returnvalue_2 (select `/Game/Game/System/Enums/EDamage` _damage :`NewEnumerator13` (struct :`TagName` "Attribute.Physical.Shield") :`NewEnumerator15` (struct :`TagName` "Attribute.Magic.Shield") :!type "GameplayTag Structure"))
    (bind _attributefound (`/Game/Game/System/Components/AC_Attributes.GetAttributeFromTag` (`local.AttributesComponent`) _returnvalue_2))
    (bind _returnvalue_3 (- (`.Curent_17_4F1F242B4B6319F1A1C212A3DDC2FAD3` (break `/Game/Game/System/Structs/FAttributeData` _attributefound)) (`local.Damage`)))
    (`/Game/Game/System/Components/AC_Attributes.ChangeAttribute` (`local.AttributesComponent`) _returnvalue_2 (`KismetMathLibrary.FMax` _returnvalue_3) "NewEnumerator6" (make `/Game/Game/System/Structs/FOrigin` _returnvalue (`/Game/Game/Blueprints/Units/BP_Unit.CommandController` (cast `/Game/Game/Blueprints/Units/BP_Unit` _returnvalue :!pure true))))
    (if (< _returnvalue_3 0.0)
      (return (`KismetMathLibrary.Abs` _returnvalue_3))
      (else
        (return 0.0)))
    (else
      (return (`local.Damage`)))))

(fn `GetTeam`
  (returns (Team :type "/Game/Game/System/Enums/ETeam Enum"))
  (return "NewEnumerator0"))

(fn `IsOwnerDead?`
  (returns (`IsDead?` :type Boolean))
  (bind _attributefound (`/Game/Game/System/Components/AC_Attributes.GetAttributeFromTag` :`self` (`Actor.GetComponentByClass` (`self.GetOwner`) "/Game/Game/System/Components/AC_Attributes.AC_Attributes_C")))
  (if (<= (`.Curent_17_4F1F242B4B6319F1A1C212A3DDC2FAD3` (break `/Game/Game/System/Structs/FAttributeData` _attributefound)) 0.0)
    (return true)
    (else
      (return false))))