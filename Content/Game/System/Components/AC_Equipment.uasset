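; AC_Equipment is an actor component that manages the weapon its owner has equipped.
; EquipWeapon removes any current weapon, spawns a BP_Weapon owned by the actor from the supplied weapon data, stores it and calls its AddAction.
; UnequipWeapon calls RemoveAction, destroys the weapon and clears the reference, which GetWeapon exposes.
; Socket attachment is left disconnected and GetCurrentEquipment is an empty stub.
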(event `self.ReceiveBeginPlay`)

(fn `EquipWeapon`
  (params (WeaponToEquip :type "/Game/Game/Blueprints/Equipment/Weapons/Data/PDA_Weapon Object Reference") (SocketName :type Name))
  (bind _returnvalue (`self.GetOwner`))
  (`/Engine/EditorBlueprintResources/StandardMacros.IsValid` (`Actor.GetComponentByClass` _returnvalue "AC_Equipment_C")
    (:`Is Valid`
      (`self.UnequipWeapon`)
      (bind _returnvalue_2 (`|SpawnActorFromClass` "/Game/Game/Blueprints/Equipment/Weapons/BP_Weapon.BP_Weapon_C" (`KismetMathLibrary.MakeTransform` (0.0 0.0 0.0)) "Undefined" "MultiplyWithRoot" _returnvalue WeaponToEquip null))
      (bind _output_get (set `self.EquippedWeapon` _returnvalue_2))
      (`/Game/Game/Blueprints/Equipment/Weapons/BP_Weapon.AddAction` _output_get))))

(fn `GetCurrentEquipment`)

(fn `GetWeapon`
  (returns (EquippedWeapon :type "/Game/Game/Blueprints/Equipment/Weapons/BP_Weapon Object Reference"))
  (return (`self.EquippedWeapon`)))

(fn `UnequipWeapon`
  (bind _equippedweapon (`self.EquippedWeapon`)
    (:`then`
      (`/Game/Game/Blueprints/Equipment/Weapons/BP_Weapon.RemoveAction` _equippedweapon)
      (`Actor.K2_DestroyActor` _equippedweapon)
      (set `self.EquippedWeapon` null))
    (:`else`)))