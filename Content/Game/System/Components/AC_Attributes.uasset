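; Attribute component holding an actor's stats, such as health, resource, damage, resist and haste, addressed by gameplay tag.
; A shared tag-switch macro routes lookups, changes and listener binding to per-attribute variables and dispatchers.
; Changes add to an attribute's Base, Delta, Multiplier or Max, then broadcast a context with value and origin.
; RepNotifies fire health or resource update events, and the authority adds random Haste at BeginPlay.
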(event `self.ReceiveBeginPlay`
  (`/Engine/EditorBlueprintResources/ActorComponentMacros.Switch Has Authority`
    (:`Authority`
      (set `self.Haste` (+ (`self.Haste`) (`KismetMathLibrary.RandomFloatInRange` 0.0 60.0))))))

(event `Signature` :!signature `self.OnAttributeHealthChange`
  (params (AttributeContext :type "/Game/Game/System/Structs/FAttributeContext Structure")))

(fn `AddAttributeListener`
  (params (AttributeTag :type "GameplayTag Structure") (Event :type "Delegate (by ref)"))
  (`self.ReturnAttributeFromTag` AttributeTag
    (:`AreaSize`
      (add `self.OnAttributeAreaSizeChange` (`local.Event`)))
    (:`Cooldown`
      (add `self.OnAttributeCooldownChange` (`local.Event`)))
    (:`Duration`
      (add `self.OnAttributeDurationChange` (`local.Event`)))
    (:`Haste`
      (add `self.OnAttributeHasteChange` (`local.Event`)))
    (:`Health`
      (add `self.OnAttributeHealthChange` (`local.Event`)))
    (:`HealthRegen`
      (add `self.OnAttributeHealthRegenChange` (`local.Event`)))
    (:`HealingPower`
      (add `self.OnAttributeHealingPowerChange` (`local.Event`)))
    (:`MagicDamage`
      (add `self.OnAttributeMagicDamageChange` (`local.Event`)))
    (:`MagicPierce`
      (add `self.OnAttributeMagicPierceChange` (`local.Event`)))
    (:`MagicResist`
      (add `self.OnAttributeMagicResistChange` (`local.Event`)))
    (:`MagicVamp`
      (add `self.OnAttributeMagicVampChange` (`local.Event`)))
    (:`PhysicalDamage`
      (add `self.OnAttributePhysicalDamageChange` (`local.Event`)))
    (:`PhysicalPierce`
      (add `self.OnAttributePhysicalPierceChange` (`local.Event`)))
    (:`PhysicalResist`
      (add `self.OnAttributePhysicalResistChange` (`local.Event`)))
    (:`PhysicalVamp`
      (add `self.OnAttributePhysicalVampChange` (`local.Event`)))
    (:`Range`
      (add `self.OnAttributeRangeChange` (`local.Event`)))
    (:`Resource`
      (add `self.OnAttributeResourceChange` (`local.Event`)))
    (:`ResourceRegen`
      (add `self.OnAttributeResourceRegenChanged` (`local.Event`)))
    (:`Tenacity`
      (add `self.OnAttributeTenacityChange` (`local.Event`)))))

(fn `Change Attribute Value`
  (params (AttributeTag :type "/Game/Game/System/Structs/FAttributeData Structure (by ref)") (Value :type "Float (double-precision)") (AttributeType :type "/Game/Game/System/Enums/EAttributes Enum" :default "NewEnumerator0"))
  (switch `/Game/Game/System/Enums/EAttributes` AttributeType
    (:`NewEnumerator1`
      (`self.UpdateAttributeBase` (`local.AttributeTag`) (`local.Value`))
      (return))
    (:`NewEnumerator2`
      (`self.UpdateAttributeDelta` (`local.AttributeTag`) (`local.Value`))
      (return))
    (:`NewEnumerator3`
      (`self.UpdateAttributeMultiplier` (`local.AttributeTag`) (`local.Value`))
      (return))
    (:`NewEnumerator4`
      (`self.UpdateAttributeMax` (`local.AttributeTag`) (`local.Value`))
      (return))))

(fn `ChangeAttribute`
  (params (AttributeTag :type "GameplayTag Structure") (Value :type "Float (double-precision)") (AttributeType :type "/Game/Game/System/Enums/EAttributes Enum" :default "NewEnumerator0") (Origin :type "/Game/Game/System/Structs/FOrigin Structure"))
  (`self.ReturnAttributeFromTag` AttributeTag
    (:`AreaSize`
      (`self.Change Attribute Value` (`self.AttributeAreaSize`) (`local.Value`) (`local.AttributeType`))
      (bind _context (`self.CreateAttributeContext` (`self.AttributeAreaSize`) (`local.Value`) (`local.Origin`)))
      (`self.OnAttributeAreaSizeChange` _context)
      (return))
    (:`Cooldown`
      (`self.Change Attribute Value` (`self.AttributeCooldown`) (`local.Value`) (`local.AttributeType`))
      (bind _context_2 (`self.CreateAttributeContext` (`self.AttributeCooldown`) (`local.Value`) (`local.Origin`)))
      (`self.OnAttributeCooldownChange` _context_2)
      (return))
    (:`Duration`
      (`self.Change Attribute Value` (`self.AttributeDuration`) (`local.Value`) (`local.AttributeType`))
      (bind _context_3 (`self.CreateAttributeContext` (`self.AttributeDuration`) (`local.Value`) (`local.Origin`)))
      (`self.OnAttributeDurationChange` _context_3)
      (return))
    (:`Haste`
      (`self.Change Attribute Value` (`self.AttributeHaste`) (`local.Value`) (`local.AttributeType`))
      (bind _context_4 (`self.CreateAttributeContext` (`self.AttributeHaste`) (`local.Value`) (`local.Origin`)))
      (`self.OnAttributeHasteChange` _context_4)
      (return))
    (:`Health`
      (`self.Change Attribute Value` (`self.AttributeHealth`) (`local.Value`) (`local.AttributeType`))
      (bind _context_5 (`self.CreateAttributeContext` (`self.AttributeHealth`) (`local.Value`) (`local.Origin`)))
      (`self.OnAttributeHealthChange` _context_5)
      (return))
    (:`HealthRegen`
      (`self.Change Attribute Value` (`self.AttributeHealthRegen`) (`local.Value`) (`local.AttributeType`))
      (bind _context_6 (`self.CreateAttributeContext` (`self.AttributeHealthRegen`) (`local.Value`) (`local.Origin`)))
      (`self.OnAttributeHealthRegenChange` _context_6)
      (return))
    (:`HealingPower`
      (`self.Change Attribute Value` (`self.AttributeHealingPower`) (`local.Value`) (`local.AttributeType`))
      (bind _context_7 (`self.CreateAttributeContext` (`self.AttributeHealingPower`) (`local.Value`) (`local.Origin`)))
      (`self.OnAttributeHealingPowerChange` _context_7)
      (return))
    (:`MagicDamage`
      (`self.Change Attribute Value` (`self.AttributeMagicDamage`) (`local.Value`) (`local.AttributeType`))
      (bind _context_8 (`self.CreateAttributeContext` (`self.AttributeMagicDamage`) (`local.Value`) (`local.Origin`)))
      (`self.OnAttributeMagicDamageChange` _context_8)
      (return))
    (:`MagicPierce`
      (`self.Change Attribute Value` (`self.AttributeMagicPierce`) (`local.Value`) (`local.AttributeType`))
      (bind _context_9 (`self.CreateAttributeContext` (`self.AttributeMagicPierce`) (`local.Value`) (`local.Origin`)))
      (`self.OnAttributeMagicPierceChange` _context_9)
      (return))
    (:`MagicResist`
      (`self.Change Attribute Value` (`self.AttributeMagicResist`) (`local.Value`) (`local.AttributeType`))
      (bind _context_10 (`self.CreateAttributeContext` (`self.AttributeMagicResist`) (`local.Value`) (`local.Origin`)))
      (`self.OnAttributeMagicResistChange` _context_10)
      (return))
    (:`MagicVamp`
      (`self.Change Attribute Value` (`self.AttributeMagicVamp`) (`local.Value`) (`local.AttributeType`))
      (bind _context_11 (`self.CreateAttributeContext` (`self.AttributeMagicVamp`) (`local.Value`) (`local.Origin`)))
      (`self.OnAttributeMagicVampChange` _context_11)
      (return))
    (:`PhysicalDamage`
      (`self.Change Attribute Value` (`self.AttributePhysicalDamage`) (`local.Value`) (`local.AttributeType`))
      (bind _context_12 (`self.CreateAttributeContext` (`self.AttributePhysicalDamage`) (`local.Value`) (`local.Origin`)))
      (`self.OnAttributePhysicalDamageChange` _context_12)
      (return))
    (:`PhysicalPierce`
      (`self.Change Attribute Value` (`self.AttributePhysicalPierce`) (`local.Value`) (`local.AttributeType`))
      (bind _context_13 (`self.CreateAttributeContext` (`self.AttributePhysicalPierce`) (`local.Value`) (`local.Origin`)))
      (`self.OnAttributePhysicalPierceChange` _context_13)
      (return))
    (:`PhysicalResist`
      (`self.Change Attribute Value` (`self.AttributePhysicalResist`) (`local.Value`) (`local.AttributeType`))
      (bind _context_14 (`self.CreateAttributeContext` (`self.AttributePhysicalResist`) (`local.Value`) (`local.Origin`)))
      (`self.OnAttributePhysicalResistChange` _context_14)
      (return))
    (:`PhysicalVamp`
      (`self.Change Attribute Value` (`self.AttributePhysicalVamp`) (`local.Value`) (`local.AttributeType`))
      (bind _context_15 (`self.CreateAttributeContext` (`self.AttributePhysicalVamp`) (`local.Value`) (`local.Origin`)))
      (`self.OnAttributePhysicalVampChange` _context_15)
      (return))
    (:`Range`
      (`self.Change Attribute Value` (`self.AttributeRange`) (`local.Value`) (`local.AttributeType`))
      (bind _context_16 (`self.CreateAttributeContext` (`self.AttributeRange`) (`local.Value`) (`local.Origin`)))
      (`self.OnAttributeRangeChange` _context_16)
      (return))
    (:`Resource`
      (`self.Change Attribute Value` (`self.AttributeResource`) (`local.Value`) (`local.AttributeType`))
      (bind _context_17 (`self.CreateAttributeContext` (`self.AttributeResource`) (`local.Value`) (`local.Origin`)))
      (`self.OnAttributeResourceChange` _context_17)
      (return))
    (:`ResourceRegen`
      (`self.Change Attribute Value` (`self.AttributeResourceRegen`) (`local.Value`) (`local.AttributeType`))
      (bind _context_18 (`self.CreateAttributeContext` (struct) (`local.Value`) (`local.Origin`)))
      (`self.OnAttributeResourceRegenChanged` _context_18)
      (return))
    (:`Tenacity`
      (`self.Change Attribute Value` (`self.AttributeTenacity`) (`local.Value`) (`local.AttributeType`))
      (bind _context_19 (`self.CreateAttributeContext` (`self.AttributeTenacity`) (`local.Value`) (`local.Origin`)))
      (`self.OnAttributeTenacityChange` _context_19)
      (return))))

(fn `CreateAttributeContext`
  (params (AttributeChanged :type "/Game/Game/System/Structs/FAttributeData Structure") (ValueChange :type "Float (double-precision)") (Origin :type "/Game/Game/System/Structs/FOrigin Structure"))
  (returns (Context :type "/Game/Game/System/Structs/FAttributeContext Structure"))
  (return (make `/Game/Game/System/Structs/FAttributeContext` AttributeChanged ValueChange Origin)))

(fn `GetAttributeFromTag`
  (params (Tag :type "GameplayTag Structure"))
  (returns (AttributeFound :type "/Game/Game/System/Structs/FAttributeData Structure"))
  (locals (Local_AttributeFound :type "/Game/Game/System/Structs/FAttributeData Structure"))
  (`self.ReturnAttributeFromTag` Tag
    (:`AreaSize`
      (set `local.Local_AttributeFound` (`self.AttributeAreaSize`)))
    (:`Cooldown`
      (set `local.Local_AttributeFound` (`self.AttributeCooldown`)))
    (:`Duration`
      (set `local.Local_AttributeFound` (`self.AttributeDuration`)))
    (:`Haste`
      (set `local.Local_AttributeFound` (`self.AttributeHaste`)))
    (:`Health`
      (set `local.Local_AttributeFound` (`self.AttributeHealth`)))
    (:`MagicDamage`
      (set `local.Local_AttributeFound` (`self.AttributeMagicDamage`)))
    (:`MagicPierce`
      (set `local.Local_AttributeFound` (`self.AttributeMagicPierce`)))
    (:`MagicResist`
      (set `local.Local_AttributeFound` (`self.AttributeMagicResist`)))
    (:`PhysicalDamage`
      (set `local.Local_AttributeFound` (`self.AttributePhysicalDamage`)))
    (:`PhysicalPierce`
      (set `local.Local_AttributeFound` (`self.AttributePhysicalPierce`)))
    (:`PhysicalResist`
      (set `local.Local_AttributeFound` (`self.AttributePhysicalResist`)))
    (:`PhysicalVamp`
      (set `local.Local_AttributeFound` (`self.AttributeMagicVamp`)))
    (:`Range`
      (set `local.Local_AttributeFound` (`self.AttributeRange`)))
    (:`Resource`
      (set `local.Local_AttributeFound` (`self.AttributeResource`))))
  (return (`local.Local_AttributeFound`)))

(fn `OnRep_Health`
  (`self.OnUpdateHealth`))

(fn `OnRep_MagicResist`
  (`self.OnUpdateHealth`))

(fn `OnRep_PhysicalResist`
  (`self.OnUpdateHealth`))

(fn `OnRep_Resource`
  (`self.OnUpdateResource`))

(fn `UpdateAttributeBase`
  (params (AttributeData :type "/Game/Game/System/Structs/FAttributeData Structure (by ref)") (NewBaseValue :type "Float (double-precision)"))
  (returns (ModifiedAttribute :type "/Game/Game/System/Structs/FAttributeData Structure (by ref)"))
  (bind _structout (setmembers `/Game/Game/System/Structs/FAttributeData` :`StructRef` AttributeData :`Base` (+ (`.Base_8_BBA0E8AF440176EB45927ABA8E8145EA` (break `/Game/Game/System/Structs/FAttributeData` AttributeData)) NewBaseValue)))
  (return _structout))

(fn `UpdateAttributeDelta`
  (params (Attribute :type "/Game/Game/System/Structs/FAttributeData Structure (by ref)") (Delta :type "Float (double-precision)"))
  (returns (ModifiedAttribute :type "/Game/Game/System/Structs/FAttributeData Structure (by ref)"))
  (locals (Local_Attribute :type "/Game/Game/System/Structs/FAttributeData Structure"))
  (bind _structout (setmembers `/Game/Game/System/Structs/FAttributeData` :`StructRef` Attribute :`Delta` (+ (`.Delta_6_D691FC9A4583460F9DC6E6B682322354` (break `/Game/Game/System/Structs/FAttributeData` Attribute)) Delta)))
  (return _structout))

(fn `UpdateAttributeMax`
  (params (StructRef :type "/Game/Game/System/Structs/FAttributeData Structure (by ref)") (Max :type "Float (double-precision)"))
  (returns (ModdifiedAttribute :type "/Game/Game/System/Structs/FAttributeData Structure (by ref)"))
  (bind _structout (setmembers `/Game/Game/System/Structs/FAttributeData` :`StructRef` StructRef :`Max` (+ (`.Max_9_CD124E43438FF31CFF85F18B45DE496A` (break `/Game/Game/System/Structs/FAttributeData` StructRef)) Max)))
  (return _structout))

(fn `UpdateAttributeMultiplier`
  (params (Attribute :type "/Game/Game/System/Structs/FAttributeData Structure (by ref)") (Multiplier :type "Float (double-precision)"))
  (returns (ModifiedAttribute :type "/Game/Game/System/Structs/FAttributeData Structure (by ref)"))
  (bind _structout (setmembers `/Game/Game/System/Structs/FAttributeData` :`StructRef` Attribute :`Multiplier` (+ (`.Multiplier_7_1B3169A546E0CBFE0FE5FE80C9C1DC89` (break `/Game/Game/System/Structs/FAttributeData` Attribute)) Multiplier)))
  (return _structout))